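; Leecher actor that plays a looping walk cycle, then switches to a looping attack animation as it latches onto the ship.
; The switch follows a one-second delay after its trigger box overlaps a component matched by a "CharacterFollow" display-name substring.
; When DestroyLeecher is set, Tick lowers a dissolve parameter on the mesh's dynamic material and destroys the actor after a delay.
; Construction creates that material and caches the Ship's skeletal mesh.
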(event OnComponentBeginOverlap(LeecherOverlappingBoxForAnimations)
  (params (OtherActor :type Actor%20Object%20Reference) (OtherComp :type Primitive%20Component%20Object%20Reference) (OtherBodyIndex :type Integer) (bFromSweep :type Boolean) (SweepResult :type Hit%20Result%20Structure%20%28by%20ref%29))
  ;[1 1 1] animations leecher - s'accroche au vaisseau
  (if (Utilities|Enum|Equal(Enum) (Utilities|String|GetSubstring (Utilities|GetDisplayName OtherComp) 9 15) "CharacterFollow")
    (Utilities|FlowControl|Delay 1.0)
    (Components|Animation|PlayAnimation (Variables|Default|GetMeshLeecher) "/Game/Character/Anim_sets/AS_Leecher/AS_Leecher02_Attack.AS_Leecher02_Attack" true)))

(event EventBeginPlay
  ;[1 1 1] animation du leecher - déplacement
  (Components|Animation|PlayAnimation (Variables|Default|GetMeshLeecher) "/Game/Character/Anim_sets/AS_Leecher/AS_Leecher02_Walkcycle.AS_Leecher02_Walkcycle" true))

(event EventTick
  (params (DeltaSeconds :type Float%20%28single-precision%29))
  (Utilities|FlowControl|Sequence
    (:then_0
      (if (Variables|Default|GetDestroyLeecher)
        (if (< 0.0 (Variables|Default|GetDissolve))
          (Variables|Default|SetDissolve (- (Variables|Default|GetDissolve) 0.05))
          (Rendering|Material|SetScalarParameterValue (Variables|Default|GetDynamic%20instance) "DissolveValue" (Variables|Default|GetDissolve) :!class /Script/Engine.MaterialInstanceDynamic)
          (Utilities|FlowControl|Delay 2.0)
          (Actor|DestroyActor))))))

(fn ConstructionScript
  (bind _returnvalue (Rendering|Material|CreateDynamicMaterialInstance (Variables|Default|GetMeshLeecher) 0 0 :!class /Script/Engine.PrimitiveComponent))
  (Variables|Default|SetDynamic%20instance _returnvalue)
  (bind _outactors (Actor|GetAllActorsOfClass "/Game/Blueprints/Ship.Ship_C"))
  (bind _asskeletalmeshcomponent (Utilities|Casting|CastToSkeletalMeshComponent (Utilities|Array|Get(acopy) (Actor|GetComponentsByClass (Utilities|Array|Get(acopy) _outactors) "/Script/Engine.SkeletalMeshComponent"))))
  (Variables|Default|SetshipSkeletalMeshReference _asskeletalmeshcomponent))