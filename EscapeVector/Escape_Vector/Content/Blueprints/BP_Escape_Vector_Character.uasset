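; First-person player character that dashes through the air between panels, launched by Fire while touching a volume or ship.
; A camera raycast picks the target, a timeline drives speed, and Tick moves the actor along a three-point spline whose midpoint A/D deflect.
; Pre-built spline meshes render the path as a beam.
; Also handles W boost and S leecher-kill items, respawn on static-mesh overlap, and a restart menu after three deaths.
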(event OnComponentBeginOverlap(CapsuleComponent)
  (params (OtherActor :type Actor%20Object%20Reference) (OtherComp :type Primitive%20Component%20Object%20Reference) (OtherBodyIndex :type Integer) (bFromSweep :type Boolean) (SweepResult :type Hit%20Result%20Structure%20%28by%20ref%29))
  ;[1 1 1] respawn if the player hits landscape, need to set Generate overlap event of meshes to true and remove 1 life
  (if (== (Utilities|GetClass OtherActor) "/Script/Engine.StaticMeshActor")
    (Class|EscapeVectorCharacter|RespawntoPanneau)
    (Development|PrintString "TouchEnvironnement" true true "(R=1.000000,G=0.715703,B=0.079022,A=1.000000)")))

(event EventTick
  (params (DeltaSeconds :type Float%20%28single-precision%29))
  (bind _endpoint (Variables|PathCalculation|GetEndPoint))
  (bind _objecthitlocation (Variables|PathRendering|GetObjectHitLocation))
  ;[1 1 1] Watch if the player has lost three times in a row
  (Variables|FramerateCalculation|SetDeltaTime DeltaSeconds)
  (Utilities|FlowControl|Sequence
    (:then_0
      ;[1 1 1] Calculate framerate
      (Variables|FramerateCalculation|Setsecond (+ (Variables|FramerateCalculation|Getsecond) (Variables|FramerateCalculation|GetDeltaTime)))
      (Variables|FramerateCalculation|SetCounter (+ (Variables|FramerateCalculation|GetCounter) 1))
      (if (> (Variables|FramerateCalculation|Getsecond) 1.0)
        (Variables|FramerateCalculation|SetFrameRate (Math|Conversions|ToFloat(Integer) (Variables|FramerateCalculation|GetCounter)))
        (Variables|FramerateCalculation|SetCounter 0)
        (Variables|FramerateCalculation|Setsecond 0.0)))
    (:then_1
      (if (>= (Variables|Default|GetiNbDead) 3.0)
        (bind _asmyhud_c (Utilities|Casting|CastToMyHUD (HUD|GetHUD (Game|GetPlayerController 0))))
        (Default|SetGametoPause _asmyhud_c)
        (Variables|/Game/Blueprints/MyHUD.MyHUD_C|SetToggleRestartMenu _asmyhud_c true)))
    (:then_2
      ;[0.4159 1 0.6296] Curve-Dash Calculation
      ;;[1 1 1] Tells if the player is not flying
      (if (or (Variables|Default|GetbVolumeTouch) (Variables|Default|GetbShipTouch))
        (if (Variables|Default|GetbShipTouch)
          (bind _outactors (Actor|GetAllActorsOfClass "/Game/Blueprints/Ship.Ship_C"))
          (Variables|PathCalculation|SetShipIgnore (Utilities|Array|Get(acopy) _outactors))
          (else
            (Variables|PathCalculation|SetShipIgnore 0)))
        ;;[1 1 1] Initialisation
        (Variables|PathCalculation|SetFlightTime 0.0)
        (Variables|PathCalculation|SetCurrentLateralForce "0, 0, 0")
        (Variables|PathCalculation|SetDeviationForce "0, 0, 0")
        (Variables|PathCalculation|SetDistance 0.0)
        (Class|SplineComponent|SetSplineWorldPoints (Variables|PathRendering|GetSpline) (Utilities|Array|MakeArray "" "" ""))
        (CallFunction|DrawCurvePath)
        (else
          ;;[1 1 1] Calculate the distance in between the start and end point of the dash
          (if (Variables|PathCalculation|GetisPanelTargeted)
            (Variables|PathCalculation|SetDistanceToDest (Math|Vector|VectorLength (- (Variables|PathRendering|GetObjectHitLocation) (Variables|PathRendering|GetStartPoint))))
            (else
              (Variables|PathCalculation|SetDistanceToDest (Math|Vector|VectorLength (- (Variables|PathCalculation|GetEndPoint) (Variables|PathRendering|GetStartPoint))))))
          (Variables|PathCalculation|SetFlightTime (+ (Variables|PathCalculation|GetFlightTime) (Variables|FramerateCalculation|GetDeltaTime)))
          (Variables|PathCalculation|SetDistance (+ (/ (+ (Math|Vector|VectorLength (Variables|PathCalculation|GetupdateVelocity)) (Variables|ActivableItems|GetactualBoost)) (Variables|FramerateCalculation|GetFrameRate)) (Variables|PathCalculation|GetDistance)))
          (Variables|PathCalculation|SetDistance%25 (/ (+ (/ (+ (Math|Vector|VectorLength (Variables|PathCalculation|GetupdateVelocity)) (Variables|ActivableItems|GetactualBoost)) (Variables|FramerateCalculation|GetFrameRate)) (Variables|PathCalculation|GetDistance)) (Variables|PathCalculation|GetDistanceToDest)))
          ;;[1 1 1] If the Player target is a panel
          (if (and (!= (Variables|PathCalculation|GetObjectHit) 0) (Variables|PathCalculation|GetisPanelTargeted))
            ;;[1 1 1] Set The spline path
            (bind _correctionpoint (CallFunction|FindCorrectiontoCurvePoint (/ (Variables|PathCalculation|GetDeviationForce) 1e+02) _objecthitlocation))
            (Class|SplineComponent|SetSplineWorldPoints (Variables|PathRendering|GetSpline) (Utilities|Array|MakeArray (Variables|PathRendering|GetStartPoint) _correctionpoint _objecthitlocation))
            (else
              (bind _correctionpoint_2 (CallFunction|FindCorrectiontoCurvePoint (/ (Variables|PathCalculation|GetDeviationForce) 1e+02) _endpoint))
              (Class|SplineComponent|SetSplineWorldPoints (Variables|PathRendering|GetSpline) (Utilities|Array|MakeArray (Variables|PathRendering|GetStartPoint) _correctionpoint_2 _endpoint))))
          ;;[1 1 1] Draw path and move the player along
          (Utilities|FlowControl|Sequence
            (:then_0
              ;;[1 1 1] Si le joueur est en plein saut et qu'il appuie sur A ou D on update les vecteurs de déviations
              (bind _returnvalue (Utilities|Casting|CastToPlayerController (Pawn|GetController)))
              (if (and (Game|Player|IsInputKeyDown _returnvalue "D") (<= (Math|Vector|VectorLength (Variables|PathCalculation|GetDeviationForce)) (Variables|PathCalculation|GetDeviationCap)))
                (CallFunction|SetDeviationForce true)
                (elif (and (<= (Math|Vector|VectorLength (Variables|PathCalculation|GetDeviationForce)) (Variables|PathCalculation|GetDeviationCap)) (Game|Player|IsInputKeyDown _returnvalue "A"))
                  (CallFunction|SetDeviationForce false))))
            (:then_1
              (Transformation|SetActorLocation (Class|SplineComponent|GetWorldLocationatDistanceAlongSpline (Variables|PathRendering|GetSpline) (Variables|PathCalculation|GetDistance)) false)
              (CallFunction|DrawCurvePath))))))
    (:then_3
      ;[1 1 1] Make sure that if you are dashing to a platform, it stays activated.
      (bind _outactors_2 (Actor|GetAllActorsOfClass "/Game/Blueprints/BlueprintPanneau.BlueprintPanneau_C"))
      (for _array_element _outactors_2
        (bind _asblueprintpanneau_c (Utilities|Casting|CastToBlueprintPanneau _array_element))
        (if (Variables|/Game/Blueprints/BlueprintPanneau.BlueprintPanneau_C|GetPlayingDashingTO _asblueprintpanneau_c)
          (Components|Animation|PlayAnimation (Variables|/Game/Blueprints/BlueprintPanneau.BlueprintPanneau_C|Get%20Panneau_Skeletal_Mesh _asblueprintpanneau_c) "/Game/Assets/panneau/panneaux_redesign/AS_panneau_activation_02.AS_panneau_activation_02" false)
          (Components|Timeline|SetPlayRate (Variables|/Game/Blueprints/BlueprintPanneau.BlueprintPanneau_C|Get%20Panneau_Skeletal_Mesh _asblueprintpanneau_c) 1.0)
          (Rendering|SetRenderCustomDepth (Variables|/Game/Blueprints/BlueprintPanneau.BlueprintPanneau_C|Get%20Panneau_Skeletal_Mesh _asblueprintpanneau_c) true))))))

(event EventIsRespawning
  ;[1 1 1] Use the RotationCamera to set the Camera when respawning and make sure we say we are not dashing to a platform.
  (Pawn|SetControlRotation (Game|GetPlayerController 0) (Variables|Default|GetRotationCamera))
  (bind _outactors (Actor|GetAllActorsOfClass "/Game/Blueprints/BlueprintPanneau.BlueprintPanneau_C"))
  (for _array_element _outactors
    (bind _asblueprintpanneau_c (Utilities|Casting|CastToBlueprintPanneau _array_element))
    (if (not (Variables|/Game/Blueprints/BlueprintPanneau.BlueprintPanneau_C|GetOnPlatform _asblueprintpanneau_c))
      (Components|Animation|PlayAnimation (Variables|/Game/Blueprints/BlueprintPanneau.BlueprintPanneau_C|Get%20Panneau_Skeletal_Mesh _asblueprintpanneau_c) "/Game/Assets/panneau/panneaux_redesign/AS_panneau_activation_02.AS_panneau_activation_02" false)
      (Components|Timeline|SetPlayRate (Variables|/Game/Blueprints/BlueprintPanneau.BlueprintPanneau_C|Get%20Panneau_Skeletal_Mesh _asblueprintpanneau_c) -1.0)
      (Rendering|SetRenderCustomDepth (Variables|/Game/Blueprints/BlueprintPanneau.BlueprintPanneau_C|Get%20Panneau_Skeletal_Mesh _asblueprintpanneau_c) false)
      (Variables|/Game/Blueprints/BlueprintPanneau.BlueprintPanneau_C|SetPlayingDashingTO _asblueprintpanneau_c false))))

(event Input|ActionEvents|InputActionFire
  (bind _firstpersoncameracomponent (Variables|Default|GetFirstPersonCameraComponent))
  (bind _multivitessedeplacement (Variables|Default|GetMultiVitesseDeplacement))
  (bind _firstpersoncameracomponent_2 (Variables|Default|GetFirstPersonCameraComponent))
  (bind _returnvalue (Transformation|GetWorldLocation _firstpersoncameracomponent))
  (bind _returnvalue_2 (+ _returnvalue "0,25.000000,-15.000000"))
  ;[1 1 1] Courbe determinant la vitesse d'un dash
  (:Pressed
    (if (or (Variables|Default|GetbVolumeTouch) (Variables|Default|GetbShipTouch))
      (Variables|Default|SetRotationCamera (Transformation|GetWorldRotation (Variables|Default|GetCapsuleComponent)) :!label _label)
      (Utilities|FlowControl|Sequence
        (:then_0
          ;[1 1 1] Var to detect when to transition animation
          (Variables|Default|SetIsDashing true)
          (Utilities|FlowControl|Delay 0.5)
          (Variables|Default|SetIsDashing false))
        (:then_1
          (Variables|PathCalculation|SetEndPoint (+ (Transformation|GetWorldLocation _firstpersoncameracomponent_2) (* (Math|Vector|GetForwardVector _firstpersoncameracomponent_2) 5e+04)))
          (Utilities|FlowControl|Sequence
            (:then_0
              (Class|EscapeVectorCharacter|OnFire)
              (Variables|PathCalculation|SetRightForce (Transformation|GetActorRightVector))
              (Variables|PathCalculation|SetStartSpeed (* (Variables|Default|GetVitesseLow) _multivitessedeplacement))
              (Variables|Default|SetPeakSpeed (* _multivitessedeplacement (Variables|Default|GetVitesseMax)))
              (Variables|PathCalculation|SetDirectionDash (Math|Vector|GetForwardVector (Variables|Default|GetFirstPersonCameraComponent)))
              (bind _newtrack_0 (Timeline|Timeline_0 PlayFromStart)
                (:Update
                  (if (Variables|Default|GetbVolumeTouch)
                    ;[1 1 1] Var to detect when to transition animation
                    (Utilities|FlowControl|Sequence
                      (:then_0
                        (Variables|Default|SetIsLanding true)
                        (Utilities|FlowControl|Delay 0.5)
                        (Variables|Default|SetIsLanding false))
                      (:then_1
                        (Timeline|Timeline_0 Stop)))
                    (else
                      (Variables|PathCalculation|SetupdateVelocity (* (Variables|PathCalculation|GetDirectionDash) (Math|Float|Lerp (Variables|PathCalculation|GetStartSpeed) (Variables|Default|GetPeakSpeed) _newtrack_0)))
                      (Class|PlayerController|ClientPlayCameraShake (Game|GetPlayerController 0) "/Game/Blueprints/CamShake.CamShake_C" 0.5 "ECameraAnimPlaySpace::CameraLocal" "0, 0, 0"))))))
            (:then_1
              ;[1 1 1] Vitesse de l'exécution de la courbe selon la distance entre deux objets. (Penser à enlever les debug string quand fini de tweak)
              (Variables|PathRendering|SetStartPoint _returnvalue_2)
              (bind (_hitresult _returnvalue_3) (CallFunction|DrawRaycastSimple (Utilities|Array|MakeArray (Variables|PathCalculation|GetObjectHit) (Variables|PathCalculation|GetActualPanel) (Variables|PathCalculation|GetShipIgnore))))
              (if _returnvalue_3
                (Variables|PathRendering|SetObjectHitLocation (.Location (Collision|BreakHitResult _hitresult)))
                (Variables|PathCalculation|SetObjectHit (.HitActor (Collision|BreakHitResult _hitresult)))
                (Variables|PathCalculation|SetisPanelTargeted true)
                (bind _asblueprintpanneau_c (Utilities|Casting|CastToBlueprintPanneau (.HitActor (Collision|BreakHitResult _hitresult))))
                (Components|Timeline|SetPlayRate (Variables|Default|GetTimeline_0) (/ 1.1 (/ (Math|Vector|VectorLength (- (.ImpactPoint (Collision|BreakHitResult _hitresult)) _returnvalue_2)) 1e+04)))
                (Variables|/Game/Blueprints/BlueprintPanneau.BlueprintPanneau_C|SetPlayingDashingTO _asblueprintpanneau_c true)
                (else
                  (Variables|PathCalculation|SetisPanelTargeted false)
                  (Components|Timeline|SetPlayRate (Variables|Default|GetTimeline_0) 1.0)))))))
      (elif (Variables|Default|GetbVolumeTouch)
        (goto _label)))))

(event Input|KeyboardEvents|W
  ;[1 1 1] Use item
  (:Pressed
    (if (Variables|ActivableItems|Getitem_speedBoost)
      (Variables|ActivableItems|Setitem_speedBoost false)
      (Variables|ActivableItems|SetactualBoost (Variables|ActivableItems|GetboostValue))
      (Variables|ActivableItems|SetisSpeedBoosted true)
      (Utilities|FlowControl|Delay (Variables|ActivableItems|GetboostDuration))
      (Variables|ActivableItems|SetactualBoost 0.0)
      (Variables|ActivableItems|SetisSpeedBoosted false))))

(event Input|KeyboardEvents|S
  ;[1 1 1] Use item
  (:Pressed
    (if (Variables|ActivableItems|Getitem_destroyAllLeechers)
      (Variables|ActivableItems|Setitem_destroyAllLeechers false)
      (bind _outactors (Actor|GetAllActorsOfClass "/Game/Blueprints/Ship.Ship_C"))
      (bind _asship_c (Utilities|Casting|CastToShip (Utilities|Array|Get(acopy) _outactors)))
      (Default|DissolveAllLeechersonShip _asship_c)
      (Development|PrintString "All Leechers has been killed!"))))

(fn ConstructionScript
  (bind _returnvalue (AddComponent|AddSplineComponent true))
  (Variables|PathRendering|SetSpline _returnvalue)
  (for _index (range 0 12)
    (bind _returnvalue_2 (AddComponent|AddSplineMeshComponent true))
    (Components|StaticMesh|SetStaticMesh _returnvalue_2 (Variables|PathRendering|GetBeam))
    (SplineMesh|SetStartScale (Utilities|Array|MakeArray _returnvalue_2) "(X=0.100000,Y=0.100000)" :!class /Script/Engine.SplineMeshComponent)
    (SplineMesh|SetEndScale (Utilities|Array|MakeArray _returnvalue_2) "(X=0.100000,Y=0.100000)" :!class /Script/Engine.SplineMeshComponent)
    (Utilities|Array|AppendArray (Variables|PathRendering|GetSplineMeshes) (Utilities|Array|MakeArray _returnvalue_2))))

(fn IsontheSameOrientation
  (params (Vector%201 :type Vector) (Vector%202 :type Vector))
  (bind _x (Math|Vector|BreakVector Vector%202))
  (bind _x_2 (Math|Vector|BreakVector Vector%201))
  (return (or (and (>= _x_2 0.0) (>= _x 0.0)) (and (<= _x_2 0.0) (<= _x 0.0)))))

(fn DrawCurvePath
  (bind _spline (Variables|PathRendering|GetSpline))
  (bind _splinemeshes (Variables|PathRendering|GetSplineMeshes))
  (for _index (range 0 (Utilities|Array|Length _splinemeshes))
    (SplineMesh|SetStartandEnd (Utilities|Array|Get(acopy) _splinemeshes _index) (Class|SplineComponent|GetWorldLocationatDistanceAlongSpline _spline (* _index 1e+03)) (* (Class|SplineComponent|GetWorldDirectionatDistanceAlongSpline _spline (* _index 1e+03)) 1e+03) (Class|SplineComponent|GetWorldLocationatDistanceAlongSpline _spline (+ (* _index 1e+03) 1e+03)) (* (Class|SplineComponent|GetWorldDirectionatDistanceAlongSpline _spline (+ (* _index 1e+03) 1e+03)) 1e+03) :!class /Script/Engine.SplineMeshComponent)))

(fn FindCorrectiontoCurvePoint
  (params (ForceToAdd :type Vector) (EndPoint :type Vector))
  (bind _startpoint (Variables|PathRendering|GetStartPoint))
  (return (+ (+ (/ (- EndPoint _startpoint) 2.0) _startpoint) ForceToAdd)))

(fn SetDeviationForce
  (params (Right :type Boolean))
  (bind _rightforce (Variables|PathCalculation|GetRightForce))
  (bind _rightforce_2 (Variables|PathCalculation|GetRightForce))
  (bind _lateralforce (Variables|PathCalculation|GetLateralForce))
  (bind _returnvalue (* _rightforce_2 _lateralforce))
  (bind _returnvalue_2 (* _lateralforce -1.0))
  (bind _returnvalue_3 (* _rightforce _returnvalue_2))
  (if Right
    (Variables|PathCalculation|SetCurrentLateralForce _returnvalue)
    (bind _isonthesameorientation (CallFunction|IsontheSameOrientation _returnvalue (Variables|PathCalculation|GetDeviationForce)))
    (if _isonthesameorientation
      (Variables|PathCalculation|SetDeviationForce (+ _returnvalue (Variables|PathCalculation|GetDeviationForce)))
      (else
        (Variables|PathCalculation|SetDeviationForce (+ _returnvalue (Variables|PathCalculation|GetDeviationForce)))))
    (else
      (Variables|PathCalculation|SetCurrentLateralForce _returnvalue_3)
      (bind _isonthesameorientation_2 (CallFunction|IsontheSameOrientation _returnvalue_3 (Variables|PathCalculation|GetDeviationForce)))
      (if _isonthesameorientation_2
        (Variables|PathCalculation|SetDeviationForce (+ _returnvalue_3 (Variables|PathCalculation|GetDeviationForce)))
        (else
          (Variables|PathCalculation|SetDeviationForce (+ _returnvalue_3 (Variables|PathCalculation|GetDeviationForce))))))))

(fn DrawRaycastSimple
  (params (ActorsToIgnore :type Array%20of%20Actor%20Object%20References))
  (bind _firstpersoncameracomponent (Variables|Default|GetFirstPersonCameraComponent))
  (bind _returnvalue (Transformation|GetWorldLocation _firstpersoncameracomponent))
  (bind _returnvalue_2 (+ _returnvalue "0,25.000000,-15.000000"))
  (bind (_outhit _returnvalue_3) (Collision|LineTraceByChannel _returnvalue_2 (+ _returnvalue_2 (* (Math|Vector|GetForwardVector (Transformation|GetWorldRotation _firstpersoncameracomponent)) 5e+04)) "TraceTypeQuery1" false ActorsToIgnore "None"))
  (return _outhit _returnvalue_3))