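; Player-boardable ship that rides a spline, drawn with spline meshes at construction, and enables leecher spawn volumes nearby.
; Leechers snap to free sockets, slowing it, reddening the beam and draining shield, then citizens; shield regenerates without leechers.
; A boarding player sticks to the nearest socket and dissolves attached leechers.
; Beamer contact or zero citizens opens the restart menu; RestartFromLastCheck rewinds to behind the checkpoint.
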(event OnComponentBeginOverlap(CharacterFollowCube)
  (params (OtherActor :type Actor%20Object%20Reference) (OtherComp :type Primitive%20Component%20Object%20Reference) (OtherBodyIndex :type Integer) (bFromSweep :type Boolean) (SweepResult :type Hit%20Result%20Structure%20%28by%20ref%29))
  (bind _self self)
  (bind _shockwave (Variables|Ship_C|GetShockwave _self))
  ;[1 1 1] If the player is on the train
  (Utilities|FlowControl|Sequence
    (:then_0
      (if (== (Game|GetPlayerCharacter 0) OtherActor)
        ;[1 1 1] activate ship's particle effect
        (Components|Activation|SetActive _shockwave true false)
        (Rendering|SetVisibility _shockwave true false)
        (Utilities|FlowControl|Delay 1.0)
        (Components|Activation|SetActive _shockwave false false)
        (Rendering|SetVisibility _shockwave true false)))
    (:then_1
      ;[1 1 1] update number of leechers on the ship
      (CallFunction|CharacterandLeecherOverlapTrain OtherActor (Variables|Default|GetShip))
      (if (Utilities|Enum|Equal(Enum) (Utilities|String|GetSubstring (Utilities|GetDisplayName OtherActor) 0 16) "LeecherBlueprint")
        (bind _asleecherblueprint_c (Utilities|Casting|CastToLeecherBlueprint OtherActor))
        (if (not (Variables|/Game/Blueprints/LeecherBlueprint.LeecherBlueprint_C|GetDestroyLeecher _asleecherblueprint_c))
          (Variables|LeechersVariables|SetNbOfLeechers (+ (Variables|LeechersVariables|GetNbOfLeechers) 1))
          (Variables|Default|SetRegen false))))))

(event OnComponentBeginOverlap(LeecherLocationSocket1)
  (params (OtherActor :type Actor%20Object%20Reference) (OtherComp :type Primitive%20Component%20Object%20Reference) (OtherBodyIndex :type Integer) (bFromSweep :type Boolean) (SweepResult :type Hit%20Result%20Structure%20%28by%20ref%29))
  (bind _leecherspeeddiminution (Variables|LeechersVariables|GetLeecherSpeedDiminution))
  (bind _basemovementspeed (Variables|ShipAttributes|GetBaseMovementSpeed))
  (bind _nbofleechers (Variables|LeechersVariables|GetNbOfLeechers))
  (bind _returnvalue (* _nbofleechers _leecherspeeddiminution))
  (bind _returnvalue_2 (- _basemovementspeed _returnvalue))
  ;[1 1 1] Les leechers dans la zone d'overlapping du ship sont assignés à un socket
  (Utilities|FlowControl|Sequence
    (:then_0
      (CallFunction|SendSocketNameandSkeletalReferencetoCode 0 OtherActor))
    (:then_1
      ;[1 1 1] Look if there is a change between lastKnow NumberofLeechers and current number. If so, reduce the speed consequently
      (for _array_element (Variables|Default|GetLeechersOnShip)
        (if (not (== (Variables|LeechersVariables|GetNbOfLeechers) (Variables|LeechersVariables|GetLastKnownNbOfLeechers)))
          (Variables|LeechersVariables|SetLastKnownNbOfLeechers _nbofleechers)
          (if (or (< _returnvalue_2 0.0) (Variables|Default|GetPaused))
            (Variables|ShipAttributes|SetCurrentMovementSpeed 0.0)
            (else
              (Variables|ShipAttributes|SetCurrentMovementSpeed _returnvalue_2))))))))

(event OnComponentBeginOverlap(LeecherLocationSocketShip)
  (params (OtherActor :type Actor%20Object%20Reference) (OtherComp :type Primitive%20Component%20Object%20Reference) (OtherBodyIndex :type Integer) (bFromSweep :type Boolean) (SweepResult :type Hit%20Result%20Structure%20%28by%20ref%29))
  (bind _leecherspeeddiminution (Variables|LeechersVariables|GetLeecherSpeedDiminution))
  (bind _basemovementspeed (Variables|ShipAttributes|GetBaseMovementSpeed))
  (bind _nbofleechers (Variables|LeechersVariables|GetNbOfLeechers))
  (bind _returnvalue (* _nbofleechers _leecherspeeddiminution))
  (bind _returnvalue_2 (- _basemovementspeed _returnvalue))
  ;[1 1 1] Les leechers dans la zone d'overlapping du ship sont assignés à un socket
  (Utilities|FlowControl|Sequence
    (:then_0
      (CallFunction|SendSocketNameandSkeletalReferencetoCode (Variables|Default|GetShip) OtherActor))
    (:then_1
      ;[1 1 1] Look if there is a change between lastKnow NumberofLeechers and current number. If so, reduce the speed consequently
      (for _array_element (Variables|Default|GetLeechersOnShip)
        (if (not (== (Variables|LeechersVariables|GetNbOfLeechers) (Variables|LeechersVariables|GetLastKnownNbOfLeechers)))
          (Variables|LeechersVariables|SetLastKnownNbOfLeechers _nbofleechers)
          (if (or (< _returnvalue_2 0.0) (Variables|Default|GetPaused))
            (Variables|ShipAttributes|SetCurrentMovementSpeed 0.0)
            (else
              (Variables|ShipAttributes|SetCurrentMovementSpeed _returnvalue_2))))))))

(event OnComponentBeginOverlap(ActivateNests)
  (params (OtherActor :type Actor%20Object%20Reference) (OtherComp :type Primitive%20Component%20Object%20Reference) (OtherBodyIndex :type Integer) (bFromSweep :type Boolean) (SweepResult :type Hit%20Result%20Structure%20%28by%20ref%29))
  ;[1 1 1] Allow the spawning of leechers of a certain volume if that volume is inside the detection sphere.
  (bind _asescape_vectorspawnleechervolume (Utilities|Casting|CastToEscape_VectorSpawnLeecherVolume OtherActor))
  (Class|EscapeVectorSpawnLeecherVolume|EnableSpawning _asescape_vectorspawnleechervolume))

(event OnComponentBeginOverlap(LeecherLocationSocket2)
  (params (OtherActor :type Actor%20Object%20Reference) (OtherComp :type Primitive%20Component%20Object%20Reference) (OtherBodyIndex :type Integer) (bFromSweep :type Boolean) (SweepResult :type Hit%20Result%20Structure%20%28by%20ref%29))
  (bind _leecherspeeddiminution (Variables|LeechersVariables|GetLeecherSpeedDiminution))
  (bind _basemovementspeed (Variables|ShipAttributes|GetBaseMovementSpeed))
  (bind _nbofleechers (Variables|LeechersVariables|GetNbOfLeechers))
  (bind _returnvalue (* _nbofleechers _leecherspeeddiminution))
  (bind _returnvalue_2 (- _basemovementspeed _returnvalue))
  ;[1 1 1] Les leechers dans la zone d'overlapping du ship sont assignés à un socket
  (Utilities|FlowControl|Sequence
    (:then_0
      (CallFunction|SendSocketNameandSkeletalReferencetoCode 0 OtherActor))
    (:then_1
      ;[1 1 1] Look if there is a change between lastKnow NumberofLeechers and current number. If so, reduce the speed consequently
      (for _array_element (Variables|Default|GetLeechersOnShip)
        (if (not (== (Variables|LeechersVariables|GetNbOfLeechers) (Variables|LeechersVariables|GetLastKnownNbOfLeechers)))
          (Variables|LeechersVariables|SetLastKnownNbOfLeechers _nbofleechers)
          (if (or (< _returnvalue_2 0.0) (Variables|Default|GetPaused))
            (Variables|ShipAttributes|SetCurrentMovementSpeed 0.0)
            (else
              (Variables|ShipAttributes|SetCurrentMovementSpeed _returnvalue_2))))))))

(event OnComponentBeginOverlap(BeamerTouchCollisionAndLeecherDestruction)
  (params (OtherActor :type Actor%20Object%20Reference) (OtherComp :type Primitive%20Component%20Object%20Reference) (OtherBodyIndex :type Integer) (bFromSweep :type Boolean) (SweepResult :type Hit%20Result%20Structure%20%28by%20ref%29))
  ;[0.5096 0.8644 1] Show the gameover Screen if the Ship encounters a Beamer
  (for _array_element (Collision|GetOverlappingActors "/Game/Blueprints/Beamer.Beamer_C" :!class /Script/Engine.Actor)
    (if (== _array_element OtherActor)
      (bind _asmyhud_c (Utilities|Casting|CastToMyHUD (HUD|GetHUD (Game|GetPlayerController 0))))
      (Default|SetGametoPause _asmyhud_c)
      (Variables|/Game/Blueprints/MyHUD.MyHUD_C|SetToggleRestartMenu _asmyhud_c true)
      (CallFunction|ResetArraysandNbLeechers))))

(event OnComponentBeginOverlap(CollisionBeamer)
  (params (OtherActor :type Actor%20Object%20Reference) (OtherComp :type Primitive%20Component%20Object%20Reference) (OtherBodyIndex :type Integer) (bFromSweep :type Boolean) (SweepResult :type Hit%20Result%20Structure%20%28by%20ref%29))
  (Utilities|FlowControl|Sequence
    (:then_1
      ;[1 1 1] Reset le nombre de civils quand le vaisseau passe en dessous du checkpoint
      (for _array_element (Collision|GetOverlappingActors "/Game/Blueprints/BP_CheckPointPanel.BP_CheckPointPanel_C" :!class /Script/Engine.Actor)
        (if (== _array_element OtherActor)
          (Variables|ShipAttributes|SetCitizen (Variables|ShipAttributes|GetDefaultCitizenValue)))))))

(event OnComponentEndOverlap(ActivateNests)
  (params (OtherActor :type Actor%20Object%20Reference) (OtherComp :type Primitive%20Component%20Object%20Reference) (OtherBodyIndex :type Integer))
  (bind _leecherspeeddiminution (Variables|LeechersVariables|GetLeecherSpeedDiminution))
  (bind _basemovementspeed (Variables|ShipAttributes|GetBaseMovementSpeed))
  (bind _nbofleechers (Variables|LeechersVariables|GetNbOfLeechers))
  (bind _returnvalue (* _nbofleechers _leecherspeeddiminution))
  (bind _returnvalue_2 (- _basemovementspeed _returnvalue))
  (Utilities|FlowControl|Sequence
    (:then_0
      ;[1 1 1] Allow the spawning of leechers of a certain volume if that volume is inside the detection sphere.
      (bind _asescape_vectorspawnleechervolume (Utilities|Casting|CastToEscape_VectorSpawnLeecherVolume OtherActor))
      (Class|EscapeVectorSpawnLeecherVolume|DisableSpawning _asescape_vectorspawnleechervolume))
    (:then_1
      ;[1 1 1] Look if there is a change between lastKnow NumberofLeechers and current number. If so, reduce the speed consequently
      (for _array_element (Variables|Default|GetLeechersOnShip)
        (if (not (== (Variables|LeechersVariables|GetNbOfLeechers) (Variables|LeechersVariables|GetLastKnownNbOfLeechers)))
          (Variables|LeechersVariables|SetLastKnownNbOfLeechers _nbofleechers)
          (if (or (< _returnvalue_2 0.0) (Variables|Default|GetPaused))
            (Variables|ShipAttributes|SetCurrentMovementSpeed 0.0)
            (else
              (Variables|ShipAttributes|SetCurrentMovementSpeed _returnvalue_2))))))))

(event EventTick
  (params (DeltaSeconds :type Float%20%28single-precision%29))
  (bind _nbofleechers (Variables|LeechersVariables|GetNbOfLeechers))
  (bind _defaultbeamcolor (Variables|BeamPathAttributes|GetdefaultBeamColor))
  (bind _returnvalue (* _nbofleechers 0.15))
  (bind (_r _g _b) (Math|Color|BreakColor _defaultbeamcolor))
  ;[1 1 1] Setting the distance where the cube should be on the spline
  (Utilities|FlowControl|Sequence
    (:then_0
      (Variables|Default|SetDeltaTime DeltaSeconds)
      (Variables|ShipAttributes|SetCurrentLocation (Transformation|GetWorldLocation (Variables|Default|GetSceneComponent)))
      (Variables|ShipAttributes|SetDistance (+ (Variables|ShipAttributes|GetDistance) (* (Variables|Default|GetDeltaTime) (Variables|ShipAttributes|GetCurrentMovementSpeed))))
      ;[1 1 1] Set current position on the spline
      (Transformation|SetWorldLocation (Variables|Default|GetShip) (Class|SplineComponent|GetWorldLocationatDistanceAlongSpline (Variables|BeamPathAttributes|GetPath) (Variables|ShipAttributes|GetDistance)) false)
      ;[1 1 1] Set current orientation on the spline
      (Transformation|SetWorldRotation (Variables|Default|GetShip) (Class|SplineComponent|GetWorldRotationatDistanceAlongSpline (Variables|BeamPathAttributes|GetPath) (Variables|ShipAttributes|GetDistance)) false)
      ;[1 1 1] Le joueur se colle au socket indiqué sur le vaisseau pour le suivre
      (Utilities|FlowControl|Sequence
        (:then_0
          ;[1 1 1] plus il y a de leechers accrochés au vaisseau, plus le beam devient rouge
          (Variables|BeamPathAttributes|SetbeamColor (Math|Conversions|ToLinearColor(Vector) (Math|Vector|MakeVector (Math|Float|Clamp(Float) (+ _r _returnvalue)) (Math|Float|Clamp(Float) (- _g _returnvalue)) (Math|Float|Clamp(Float) (- _b _returnvalue)))))
          (Rendering|Material|SetVectorParameterValue "/Game/Materials/MPC_Beam.MPC_Beam" "Beam_exterieur_Tint" (Variables|BeamPathAttributes|GetbeamColor) :!class /Script/Engine.KismetMaterialLibrary)
          (Rendering|Material|SetVectorParameterValue "/Game/Materials/MPC_Beam.MPC_Beam" "Beam_interieur_Tint" (Variables|BeamPathAttributes|GetbeamColor) :!class /Script/Engine.KismetMaterialLibrary))
        (:then_1
          (bind _asescape_vectorcharacter (Utilities|Casting|CastToEscape_VectorCharacter (Game|GetPlayerCharacter 0)))
          (if (Variables|/Script/Escape_Vector.Escape_VectorCharacter|GetbShipTouch _asescape_vectorcharacter)
            (Transformation|SetActorLocation (Game|GetPlayerCharacter 0) (Transformation|GetSocketLocation (Variables|Default|GetTrainPart) (Variables|Default|GetShortSocketName)) false)))))
    (:then_1
      ;[1 1 1] If Citizen Reach 0 then Restart From Last CheckPoint
      (if (<= (Variables|ShipAttributes|GetCitizen) 0)
        (bind _asmyhud_c (Utilities|Casting|CastToMyHUD (HUD|GetHUD (Game|GetPlayerController 0))))
        (Default|SetGametoPause _asmyhud_c)
        (Variables|/Game/Blueprints/MyHUD.MyHUD_C|SetToggleRestartMenu _asmyhud_c true)
        (CallFunction|ResetArraysandNbLeechers)
        (else
          ;[1 1 1] Decrease Shieldand Citizen depending on how many leechers there is on the ship
          (Variables|LeechersVariables|SetTimeCounter (+ (Variables|LeechersVariables|GetTimeCounter) (Variables|Default|GetDeltaTime)))
          (if (< (Variables|LeechersVariables|GetTimeBetweenDecrease) (Variables|LeechersVariables|GetTimeCounter))
            (Variables|ShipAttributes|SetShield (- (Variables|ShipAttributes|GetShield) (* (Math|Conversions|ToFloat(Integer) (/ (Variables|LeechersVariables|GetNbOfLeechers) 2)) (Variables|LeechersVariables|GetLeecherDamage))))
            (if (< (Variables|ShipAttributes|GetShield) 0.0)
              (Variables|ShipAttributes|SetShield 0.0)
              (Utilities|FlowControl|Delay (Variables|LeechersVariables|GetcitizenDecreaseDelay))
              (Variables|ShipAttributes|SetCitizen (- (Variables|ShipAttributes|GetCitizen) (Math|Float|Floor (* (/ (Variables|LeechersVariables|GetNbOfLeechers) 2) (Variables|LeechersVariables|GetcitizenKilledPerLeecher)))))
              (Variables|LeechersVariables|SetTimeCounter 0.0))))))
    (:then_2
      ;[1 1 1] If we reach 0 leecher, we can allow the regen
      (if (> (Variables|LeechersVariables|GetNbOfLeechers) 0)
        (Variables|Default|SetRegen false)
        (else
          (Utilities|FlowControl|Delay (Variables|ShipAttributes|GetTimeBeforeShieldStartstoRecover))
          (Variables|Default|SetRegen true))))
    (:then_3
      ;[1 1 1] Regen the shield each X seconds for Y amount.
      (if (Variables|Default|GetRegen)
        (Utilities|FlowControl|Delay (Variables|LeechersVariables|GetRegenRate))
        (if (< (Variables|ShipAttributes|GetShield) (Variables|ShipAttributes|GetMaxShield))
          (Variables|ShipAttributes|SetShield (+ (Variables|ShipAttributes|GetShield) (Variables|LeechersVariables|GetRegenValue))))))))

(event Input|KeyboardEvents|L
  ;[1 0.3407 0.2545] Debuging Stuff
  ;;[1 1 1] Met le jeu en pause en appuyant sur L
  (:Pressed
    (if (Variables|Default|GetPaused)
      (Variables|Default|SetPaused false)
      (Variables|ShipAttributes|SetCurrentMovementSpeed 5e+02)
      (else
        (Variables|Default|SetPaused true)
        (Variables|ShipAttributes|SetCurrentMovementSpeed 0.0)))))

(fn ConstructionScript
  (bind _path (Variables|BeamPathAttributes|GetPath))
  (bind _spacing (Variables|BeamPathAttributes|GetSpacing))
  (bind _scale_tangent (Variables|BeamPathAttributes|GetScale%20Tangent))
  (for _index (range 0 (.ReturnValue (Math|Float|Division(WholeandRemainder) (Spline|GetSplineLength _path) _spacing)))
    (bind _returnvalue (AddComponent|AddSplineMeshComponent true))
    (Collision|SetCollisionEnabled _returnvalue "NoCollision")
    (Components|StaticMesh|SetStaticMesh _returnvalue (Variables|BeamPathAttributes|GetBeam))
    (SplineMesh|SetStartandEnd _returnvalue (Class|SplineComponent|GetWorldLocationatDistanceAlongSpline _path (* _index _spacing)) (* (Class|SplineComponent|GetWorldDirectionatDistanceAlongSpline _path (* _index _spacing)) _scale_tangent) (Class|SplineComponent|GetWorldLocationatDistanceAlongSpline _path (+ (* _index _spacing) _spacing)) (* (Class|SplineComponent|GetWorldDirectionatDistanceAlongSpline _path (+ (* _index _spacing) _spacing)) _scale_tangent) :!class /Script/Engine.SplineMeshComponent)))

(fn RestartfromLastCheck
  (Variables|ShipAttributes|SetDistance 0.0)
  (Variables|ShipAttributes|SetShield (Variables|ShipAttributes|GetMaxShield))
  (Variables|ShipAttributes|SetCitizen (Variables|ShipAttributes|GetDefaultCitizenValue))
  (Variables|ShipAttributes|SetDistance (Math|Float|Clamp(Float) (- (Variables|ShipAttributes|GetCheckpointDistance) (Variables|ShipAttributes|GetReculCheckpoint)) (Variables|ShipAttributes|GetDeploymentLength) 1e+07))
  (CallFunction|ResetArraysandNbLeechers)
  (bind _asbp_escape_vector_character_c (Utilities|Casting|CastToBP_Escape_Vector_Character (Game|GetPlayerCharacter 0)))
  (Variables|/Script/Escape_Vector.Escape_VectorCharacter|SetbShipTouch _asbp_escape_vector_character_c false))

(fn GetNearestSocketName
  (params (targetActor :type Actor%20Object%20Reference) (closestMesh :type Skeletal%20Mesh%20Component%20Object%20Reference))
  (Variables|Default|SetShortDistanceSocket 5e+03)
  (for _array_element (Transformation|GetAllSocketNames closestMesh)
    (if (not (Utilities|Array|ContainsItem (Variables|Default|GetOccupiedSockets) _array_element))
      (if (< (Math|Vector|VectorLength (- (Transformation|GetActorLocation targetActor) (Transformation|GetSocketLocation closestMesh _array_element))) (Variables|Default|GetShortDistanceSocket))
        (Variables|Default|SetShortDistanceSocket (Math|Vector|VectorLength (- (Transformation|GetActorLocation targetActor) (Transformation|GetSocketLocation closestMesh _array_element))))
        (return _array_element closestMesh)))))

(fn GetNearestSocketNameforPlayer
  (params (NewParam :type Skeletal%20Mesh%20Component%20Object%20Reference))
  (Variables|Default|SetShortDistanceSocket 5e+03)
  (for _array_element (Transformation|GetAllSocketNames NewParam)
    (if (< (Math|Vector|VectorLength (- (Transformation|GetActorLocation (Game|GetPlayerCharacter 0)) (Transformation|GetSocketLocation NewParam _array_element))) (Variables|Default|GetShortDistanceSocket))
      (Variables|Default|SetShortDistanceSocket (Math|Vector|VectorLength (- (Transformation|GetActorLocation (Game|GetPlayerCharacter 0)) (Transformation|GetSocketLocation NewParam _array_element))))
      (Variables|Default|SetTrainPart NewParam)
      (return _array_element))))

(fn ResetArraysandNbLeechers
  (bind _leechersonship (Variables|Default|GetLeechersOnShip))
  (Utilities|Array|Clear (Variables|Default|GetOccupiedSockets))
  (for _array_element _leechersonship
    (Actor|DestroyActor _array_element))
  (Utilities|Array|Clear _leechersonship)
  (Variables|LeechersVariables|SetNbOfLeechers 0)
  (Variables|LeechersVariables|SetLastKnownNbOfLeechers 0)
  (Variables|ShipAttributes|SetCurrentMovementSpeed (Variables|ShipAttributes|GetBaseMovementSpeed)))

(fn DissolveAllLeechersonShip
  (bind _leechersonship (Variables|Default|GetLeechersOnShip))
  (Utilities|Array|Clear (Variables|Default|GetOccupiedSockets))
  (for _array_element _leechersonship
    (Variables|/Game/Blueprints/LeecherBlueprint.LeecherBlueprint_C|SetDestroyLeecher _array_element true))
  (Utilities|Array|Clear _leechersonship)
  (Variables|LeechersVariables|SetNbOfLeechers 0)
  (Variables|LeechersVariables|SetLastKnownNbOfLeechers 0)
  (Variables|ShipAttributes|SetCurrentMovementSpeed (Variables|ShipAttributes|GetBaseMovementSpeed)))

(fn AddLeecherstoLists
  (params (overlappingActor :type Actor%20Object%20Reference))
  (bind _leechersonship (Variables|Default|GetLeechersOnShip))
  (if (Utilities|Enum|Equal(Enum) (Utilities|String|GetSubstring (Utilities|GetDisplayName overlappingActor) 0 16) "LeecherBlueprint")
    (bind _asleecherblueprint_c (Utilities|Casting|CastToLeecherBlueprint overlappingActor))
    (Variables|Default|SetinList false)
    (for _array_element _leechersonship
      (if (== _array_element overlappingActor)
        (Variables|Default|SetinList true)))
    (if (not (Variables|Default|GetinList))
      (Utilities|Array|Add _leechersonship _asleecherblueprint_c))))

(fn StickPlayertoSocketandDissolveLeechers
  (params (overlappingActor :type Actor%20Object%20Reference) (NewParam :type Skeletal%20Mesh%20Component%20Object%20Reference))
  (bind _returnvalue (Game|GetPlayerCharacter 0))
  (if (== _returnvalue overlappingActor)
    (bind _asescape_vectorcharacter (Utilities|Casting|CastToEscape_VectorCharacter _returnvalue))
    (Class|EscapeVectorCharacter|TouchShip _asescape_vectorcharacter)
    (bind _nearestsocketnameforplayer (CallFunction|GetNearestSocketNameforPlayer NewParam))
    (Variables|Default|SetShortSocketName _nearestsocketnameforplayer)
    (CallFunction|DissolveAllLeechersonShip)
    (Utilities|Array|Add (Variables|Default|GetOccupiedSockets) _nearestsocketnameforplayer)))

(fn CharacterandLeecherOverlapTrain
  (params (overlappingActor :type Actor%20Object%20Reference) (skelMesh :type Skeletal%20Mesh%20Component%20Object%20Reference))
  ;[1 1 1] le joueur suit le vaisseau
  (if (== (Game|GetPlayerCharacter 0) overlappingActor)
    (bind _asescape_vectorcharacter (Utilities|Casting|CastToEscape_VectorCharacter (Game|GetPlayerCharacter 0)))
    (Class|EscapeVectorCharacter|TouchShip _asescape_vectorcharacter)
    (bind _nearestsocketnameforplayer (CallFunction|GetNearestSocketNameforPlayer skelMesh))
    (Variables|Default|SetShortSocketName _nearestsocketnameforplayer)
    ;[1 1 1] détruit les leechers sur le ship
    (CallFunction|DissolveAllLeechersonShip)
    (Utilities|Array|Add (Variables|Default|GetOccupiedSockets) _nearestsocketnameforplayer)))

(fn SendSocketNameandSkeletalReferencetoCode
  (params (skeletalReference :type Skeletal%20Mesh%20Component%20Object%20Reference) (otherActor :type Actor%20Object%20Reference))
  (bind _leechersonship (Variables|Default|GetLeechersOnShip))
  (Utilities|FlowControl|Sequence
    (:then_0
      ;[1 1 1] ajoute les leechers présents dans une liste
      (if (Utilities|Enum|Equal(Enum) (Utilities|String|GetSubstring (Utilities|GetDisplayName otherActor) 0 16) "LeecherBlueprint")
        (bind _asleecherblueprint_c (Utilities|Casting|CastToLeecherBlueprint otherActor))
        (Variables|Default|SetinList false)
        (for _array_element _leechersonship
          (if (== _array_element _asleecherblueprint_c)
            (Variables|Default|SetinList true)))
        (if (not (Variables|Default|GetinList))
          (Utilities|Array|Add _leechersonship _asleecherblueprint_c))))
    (:then_1
      (for _array_element_2 (Collision|GetOverlappingActors "/Game/Blueprints/LeecherBlueprint.LeecherBlueprint_C" :!class /Script/Engine.Actor)
        (if (== _array_element_2 otherActor)
          (bind (_nearestsocketname _closestskeletalmeshref) (CallFunction|GetNearestSocketName otherActor skeletalReference))
          (Utilities|Array|Add (Variables|Default|GetOccupiedSockets) _nearestsocketname)
          (bind _asescape_vectorleecherpawn (Utilities|Casting|CastToEscape_VectorLeecherPawn _array_element_2))
          (if (Utilities|Enum|Equal(Enum) (Utilities|String|ToString(Name) (Variables|/Script/Escape_Vector.Escape_VectorLeecherPawn|GetSocketName _asescape_vectorleecherpawn)) "None")
            (Variables|/Script/Escape_Vector.Escape_VectorLeecherPawn|SetshipSkeletalMeshReference _asescape_vectorleecherpawn _closestskeletalmeshref)
            (Variables|/Script/Escape_Vector.Escape_VectorLeecherPawn|SetSocketName _asescape_vectorleecherpawn _nearestsocketname)
            (Variables|Default|SetRegen false)))))))

(fn GetShipCitizen
  (return (Variables|ShipAttributes|GetCitizen)))

(fn GetShipShield
  (return (Variables|ShipAttributes|GetShield) (Variables|ShipAttributes|GetMaxShield)))

(fn GetShipSpeed
  (return (Variables|ShipAttributes|GetCurrentMovementSpeed)))