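; Main menu HUD that draws a background with Play Demo and Quit buttons, loading the LDTest level or quitting the game.
; DrawHUD renders each button through DrawButton, which adds a named hitbox and roughly centered label.
; Hitbox events swap hover and click textures, and releasing Play shows loading text briefly before opening the level.
; BeginPlay enables mouse interaction and disables controller input; the Level 2 button's draw call is disconnected.
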(event EventHitBoxRelease
  (params (BoxName :type Name :default "None"))
  (switch name BoxName
    (:level1
      (Variables|Default|SetToggle%20LoadingScreen true)
      (Utilities|FlowControl|Delay 0.1)
      (Game|OpenLevel(byName) "LDTest"))
    (:Level2
      (Variables|Default|SetToggle%20LoadingScreen true)
      (Utilities|FlowControl|Delay 0.1)
      (Variables|Default|SetToggle%20LoadingScreen false))
    (:Quit
      (Game|QuitGame))))

(event EventBeginPlay
  (bind _returnvalue (Game|GetPlayerController 0))
  (Variables|/Script/Engine.PlayerController|SetbShowMouseCursor _returnvalue true)
  (Variables|/Script/Engine.PlayerController|SetbEnableMouseOverEvents _returnvalue true)
  (Variables|/Script/Engine.PlayerController|SetbEnableClickEvents _returnvalue true)
  (Input|DisableInput _returnvalue _returnvalue)
  (Input|SetIgnoreLookInput _returnvalue true))

(event EventDrawHUD
  (params (SizeX :type Integer) (SizeY :type Integer))
  (bind _level1_buttontexture (Variables|Default|GetLevel1_ButtonTexture))
  (Variables|Default|SetScreenDimensions (Math|Vector2D|MakeVector2D (Math|Conversions|ToFloat(Integer) SizeX) (Math|Conversions|ToFloat(Integer) SizeY)))
  (Canvas|DrawTexture (Variables|Default|GetBackgroundTexture) 0.0 0.0 (.X (Math|Vector2D|BreakVector2D (Variables|Default|GetScreenDimensions))) (.Y (Math|Vector2D|BreakVector2D (Variables|Default|GetScreenDimensions))) 0.0 0.0 1.0 1.0 "(R=1.000000,G=1.000000,B=1.000000,A=1.000000)")
  (if (Variables|Default|GetToggle%20LoadingScreen)
    (HUD|DrawText "Loading..." (Variables|Default|GetFontColor) (- (.X (Math|Vector2D|BreakVector2D (/ (Variables|Default|GetScreenDimensions) 2.0))) 7e+01) (+ (.Y (Math|Vector2D|BreakVector2D (/ (Variables|Default|GetScreenDimensions) 2.0))) 3e+02) (Variables|Default|GetFont) 1.0 false)
    (else
      (CallFunction|DrawButton _level1_buttontexture (Math|Vector2D|MakeVector2D (- (/ (.X (Math|Vector2D|BreakVector2D (Variables|Default|GetScreenDimensions))) 2.0) (Math|Conversions|ToFloat(Integer) (/ (Class|Texture2D|BlueprintGetSizeX _level1_buttontexture) 2))) (- (- (/ (.Y (Math|Vector2D|BreakVector2D (Variables|Default|GetScreenDimensions))) 2.0) (Math|Conversions|ToFloat(Integer) (/ (Class|Texture2D|BlueprintGetSizeY _level1_buttontexture) 2))) 1e+02)) "level1" "Play Demo")
      (CallFunction|DrawButton (Variables|Default|GetQuit_ButtonTexture) (Math|Vector2D|MakeVector2D (- (/ (.X (Math|Vector2D|BreakVector2D (Variables|Default|GetScreenDimensions))) 2.0) (Math|Conversions|ToFloat(Integer) (/ (Class|Texture2D|BlueprintGetSizeX _level1_buttontexture) 2))) (+ (+ (- (- (/ (.Y (Math|Vector2D|BreakVector2D (Variables|Default|GetScreenDimensions))) 2.0) (Math|Conversions|ToFloat(Integer) (/ (Class|Texture2D|BlueprintGetSizeY _level1_buttontexture) 2))) 1e+02) 1e+02) 1e+02)) "quit" "Quit"))))

(event EventHitBoxBeginCursorOver
  (params (BoxName :type Name :default "None"))
  (bind _buttonhovertexture (Variables|Default|GetButtonHoverTexture))
  (switch name BoxName
    (:level1
      (Variables|Default|SetLevel1_ButtonTexture _buttonhovertexture))
    (:Level2
      (Variables|Default|SetLevel2_ButtonTexture _buttonhovertexture))
    (:Quit
      (Variables|Default|SetQuit_ButtonTexture _buttonhovertexture))))

(event EventHitBoxEndCursorOver
  (params (BoxName :type Name :default "None"))
  (bind _buttontexture (Variables|Default|GetButtonTexture))
  (switch name BoxName
    (:level1
      (Variables|Default|SetLevel1_ButtonTexture _buttontexture))
    (:Level2
      (Variables|Default|SetLevel2_ButtonTexture _buttontexture))
    (:Quit
      (Variables|Default|SetQuit_ButtonTexture _buttontexture))))

(event EventHitBoxClick
  (params (BoxName :type Name :default "None"))
  (bind _buttonclicktexture (Variables|Default|GetButtonClickTexture))
  (switch name BoxName
    (:level1
      (Variables|Default|SetLevel1_ButtonTexture _buttonclicktexture))
    (:Level2
      (Variables|Default|SetLevel2_ButtonTexture _buttonclicktexture))
    (:Quit
      (Variables|Default|SetQuit_ButtonTexture _buttonclicktexture))))

(fn ConstructionScript)

(fn DrawButton
  (params (Texture :type Texture%202D%20Object%20Reference) (Position :type Vector%202D%20Structure) (HitBoxName :type Name) (Text :type String))
  (bind _returnvalue (Class|Texture2D|BlueprintGetSizeX Texture))
  (bind _returnvalue_2 (Class|Texture2D|BlueprintGetSizeY Texture))
  (bind (_x _y) (Math|Vector2D|BreakVector2D Position))
  (bind _returnvalue_3 (Math|Conversions|ToFloat(Integer) _returnvalue))
  (bind _returnvalue_4 (Math|Conversions|ToFloat(Integer) _returnvalue_2))
  (bind _returnvalue_5 (Math|Vector2D|MakeVector2D _returnvalue_3 _returnvalue_4))
  (bind _returnvalue_6 (/ _returnvalue_5 2.0))
  (bind _returnvalue_7 (+ Position _returnvalue_6))
  (bind (_x_2 _y_2) (Math|Vector2D|BreakVector2D _returnvalue_7))
  (Class|HUD|DrawTextureSimple Texture _x _y 1.0 false)
  (Class|HUD|AddHitBox Position _returnvalue_5 HitBoxName false)
  (HUD|DrawText Text (Variables|Default|GetFontColor) (- _x_2 (* (Utilities|String|Len Text) 7.5)) (- _y_2 2e+01) (Variables|Default|GetFont) 1.0 false))