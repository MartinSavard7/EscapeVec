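; Checkpoint panel actor that registers player progress when the Ship enters its detection range.
; Ship overlap resets the character's death count, passes it the panel mesh and checkpoint number, and saves the ship's current distance as its checkpoint distance.
; Character contact with the panel box hands over the mesh and calls TouchPanneau.
; Leaving the box plays the activation animation in reverse after a delay, gated by an OnPlatform flag.
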(event OnComponentBeginOverlap(ShipDetectionRange)
  (params (OtherActor :type Actor%20Object%20Reference) (OtherComp :type Primitive%20Component%20Object%20Reference) (OtherBodyIndex :type Integer) (bFromSweep :type Boolean) (SweepResult :type Hit%20Result%20Structure%20%28by%20ref%29))
  (bind _overlappingactors (Collision|GetOverlappingActors "/Game/Blueprints/Ship.Ship_C" :!class /Script/Engine.Actor))
  (bind _item (Utilities|Array|Get(acopy) _overlappingactors))
  ;[1 1 1] Reset the new Checkpoint settings if the ship enters the Ship DetectionRadius
  (if (== OtherActor _item)
    (bind _asbp_escape_vector_character_c (Utilities|Casting|CastToBP_Escape_Vector_Character (Game|GetPlayerCharacter 0)))
    (Variables|/Script/Escape_Vector.Escape_VectorCharacter|SetiNbDead _asbp_escape_vector_character_c 0.0)
    (Variables|/Script/Escape_Vector.Escape_VectorCharacter|SetcheckPointSkeletalRef _asbp_escape_vector_character_c (Variables|Default|Get%20Panneau_Skeletal_Mesh))
    (Variables|/Game/Blueprints/BP_Escape_Vector_Character.BP_Escape_Vector_Character_C|SetCheckPointNumber _asbp_escape_vector_character_c (Variables|Default|GetCheckpoint%20number))
    (bind _asship_c (Utilities|Casting|CastToShip _item))
    (Variables|/Game/Blueprints/Ship.Ship_C|SetCheckpointDistance _asship_c (Variables|/Game/Blueprints/Ship.Ship_C|GetDistance _asship_c))))

(event OnComponentBeginOverlap(PanelCollisionBox)
  (params (OtherActor :type Actor%20Object%20Reference) (OtherComp :type Primitive%20Component%20Object%20Reference) (OtherBodyIndex :type Integer) (bFromSweep :type Boolean) (SweepResult :type Hit%20Result%20Structure%20%28by%20ref%29))
  (bind _asescape_vectorcharacter (Utilities|Casting|CastToEscape_VectorCharacter OtherActor))
  (Variables|/Script/Escape_Vector.Escape_VectorCharacter|SetpanneauSkeletalMeshReference _asescape_vectorcharacter (Variables|Default|Get%20Panneau_Skeletal_Mesh))
  (Class|EscapeVectorCharacter|TouchPanneau _asescape_vectorcharacter))

(event OnComponentEndOverlap(PanelCollisionBox)
  (params (OtherActor :type Actor%20Object%20Reference) (OtherComp :type Primitive%20Component%20Object%20Reference) (OtherBodyIndex :type Integer))
  (bind __panneau_skeletal_mesh (Variables|Default|Get%20Panneau_Skeletal_Mesh))
  (Variables|Default|SetOnPlatform false)
  (Utilities|FlowControl|Delay 4.0)
  (if (not (Variables|Default|GetOnPlatform))
    (Components|Animation|PlayAnimation __panneau_skeletal_mesh "/Game/Assets/panneau/AS_panneau_activation.AS_panneau_activation" false)
    (Components|Timeline|SetPlayRate __panneau_skeletal_mesh -1.0)))

(fn ConstructionScript)

(fn NewFunction)