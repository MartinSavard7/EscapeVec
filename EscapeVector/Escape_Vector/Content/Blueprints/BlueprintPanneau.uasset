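; Panel actor that activates when the Escape Vector character overlaps it and retracts after the character leaves.
; Begin overlap passes its skeletal mesh and itself to the character, calls TouchPanneau, plays the activation animation and enables custom depth.
; End overlap clears OnPlatform and waits briefly, then, if the flag is still false, reverses the animation, disables custom depth and resets PlayingDashingTO.
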(event EventActorBeginOverlap
  (params (OtherActor :type Actor%20Object%20Reference))
  (bind __panneau_skeletal_mesh (Variables|Default|Get%20Panneau_Skeletal_Mesh))
  (bind _asescape_vectorcharacter (Utilities|Casting|CastToEscape_VectorCharacter OtherActor))
  (Variables|/Script/Escape_Vector.Escape_VectorCharacter|SetpanneauSkeletalMeshReference _asescape_vectorcharacter (Variables|Default|Get%20Panneau_Skeletal_Mesh))
  (Class|EscapeVectorCharacter|TouchPanneau _asescape_vectorcharacter)
  (bind _asbp_escape_vector_character_c (Utilities|Casting|CastToBP_Escape_Vector_Character OtherActor))
  (Variables|/Game/Blueprints/BP_Escape_Vector_Character.BP_Escape_Vector_Character_C|SetActualPanel _asbp_escape_vector_character_c self)
  (Components|Animation|PlayAnimation __panneau_skeletal_mesh "/Game/Assets/panneau/panneaux_redesign/AS_panneau_activation_02.AS_panneau_activation_02" false)
  (Components|Timeline|SetPlayRate __panneau_skeletal_mesh 1.0)
  (Rendering|SetRenderCustomDepth __panneau_skeletal_mesh true))

(event EventActorEndOverlap
  (params (OtherActor :type Actor%20Object%20Reference))
  (bind __panneau_skeletal_mesh (Variables|Default|Get%20Panneau_Skeletal_Mesh))
  (Variables|Default|SetDelayCompleted false)
  (Variables|Default|SetOnPlatform false)
  (Utilities|FlowControl|Delay 4.0)
  (Variables|Default|SetDelayCompleted true)
  (if (not (Variables|Default|GetOnPlatform))
    (Components|Animation|PlayAnimation __panneau_skeletal_mesh "/Game/Assets/panneau/panneaux_redesign/AS_panneau_activation_02.AS_panneau_activation_02" false)
    (Components|Timeline|SetPlayRate __panneau_skeletal_mesh -1.0)
    (Rendering|SetRenderCustomDepth __panneau_skeletal_mesh false)
    (Variables|Default|SetPlayingDashingTO false)))

(fn ConstructionScript)

(fn NewFunction)