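; HUD for Escape Vector that draws the helmet overlay, ship shield and citizens, deaths, Beamer kills, item indicators, messages and crosshair.
; Hitbox buttons drive pause and restart menus; Retry respawns the player, restores the ship and checkpoint-filtered Beamers, and removes Leechers.
; DrawHUD also scans nearby panels every frame, using screen projection to highlight, animate and flag them, with a line-of-sight trace before activation.
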(event EventHitBoxRelease
  (params (BoxName :type Name :default "None"))
  (switch name BoxName
    (:Retry
      (CallFunction|SetGametoUnPause)
      (bind _asbp_escape_vector_character_c (Utilities|Casting|CastToBP_Escape_Vector_Character (Game|GetPlayerCharacter 0)))
      (Class|EscapeVectorCharacter|RespawntoCheckPoint _asbp_escape_vector_character_c)
      (bind _outactors (Actor|GetAllActorsOfClass "/Game/Blueprints/Ship.Ship_C"))
      (bind _asship_c (Utilities|Casting|CastToShip (Utilities|Array|Get(acopy) _outactors)))
      (Default|RestartfromLastCheck _asship_c)
      (Utilities|FlowControl|Delay 0.025)
      (CallFunction|RespawnBeamerCheckpoint)
      (bind _outactors_2 (Actor|GetAllActorsOfClass "/Game/Blueprints/LeecherBlueprint.LeecherBlueprint_C"))
      (for _array_element _outactors_2
        (Actor|DestroyActor _array_element)))
    (:Quit
      (Game|QuitGame (Game|GetPlayerController 0)))
    (:ReturnToMain
      (Game|OpenLevel(byName) "MenuLevel"))
    (:Resume
      (CallFunction|SetGametoUnPause))))

(event EventDrawHUD
  (params (SizeX :type Integer) (SizeY :type Integer))
  (bind _font (Variables|Default|GetFont))
  (bind _messagelog (Variables|Default|GetMessageLog))
  (Variables|Default|SetScreenDimensions (Math|Vector2D|MakeVector2D (Math|Conversions|ToFloat(Integer) SizeX) (Math|Conversions|ToFloat(Integer) SizeY)))
  ;[1 1 1] Draw Helmet on screen
  (Utilities|FlowControl|Sequence
    (:then_0
      (Canvas|DrawTexture "/Game/Textures/HUD/T_HUD.T_HUD" 0.0 0.0 (.X (Math|Vector2D|BreakVector2D (Variables|Default|GetScreenDimensions))) (.Y (Math|Vector2D|BreakVector2D (Variables|Default|GetScreenDimensions))) 0.0 0.0 1.0 1.0 (Utilities|Struct|MakeLinearColor 1.0 1.0 1.0 1.0) "BLEND_Translucent" 1.0 true)
      ;[1 1 1] Toggle restart or Pause Menu
      (if (Variables|Default|GetToggleRestartMenu)
        (CallFunction|DrawRestartMenu)
        (elif (Variables|Default|GetTogglePauseMenu)
          (CallFunction|DrawPauseMenu)
          (else
            ;[1 1 1] Draw crosshair in center of the screen
            (CallFunction|DrawCrosshair (Variables|Default|Getcrosshair))
            ;[1 1 1] Draw Shield and Citizen of the ship to screen
            (bind _outactors (Actor|GetAllActorsOfClass "/Game/Blueprints/Ship.Ship_C"))
            (bind (_shield _maxshield) (Class|MyHUDInterface|GetShipShield(Message) (Utilities|Array|Get(acopy) _outactors)))
            (CallFunction|DrawDynamicBar (Variables|Default|GetShieldDynamicBar) "CurrentShield" (/ _shield _maxshield) _maxshield (Math|Vector2D|MakeVector2D (- (/ (.X (Math|Vector2D|BreakVector2D (Variables|Default|GetScreenDimensions))) 2.0) 197.0) (/ (.Y (Math|Vector2D|BreakVector2D (Variables|Default|GetScreenDimensions))) 7e+01)))
            (bind _citizen (Class|MyHUDInterface|GetShipCitizen(Message) (Utilities|Array|Get(acopy) _outactors)))
            (HUD|DrawText (Utilities|String|ToString(Integer) _citizen) (Variables|Default|GetFontColor) (/ (.X (Math|Vector2D|BreakVector2D (Variables|Default|GetScreenDimensions))) 1.95) (/ (.Y (Math|Vector2D|BreakVector2D (Variables|Default|GetScreenDimensions))) 5.1) (Variables|Default|GetFont) 0.7 true)
            ;[1 1 1] Draw number of death to the screen
            (bind _asescape_vectorcharacter (Utilities|Casting|CastToEscape_VectorCharacter (Game|GetPlayerCharacter 0)))
            (HUD|DrawText (Utilities|String|Append " Deaths: " (Utilities|String|ToString(Integer) (Math|Float|Floor (Variables|/Script/Escape_Vector.Escape_VectorCharacter|GetiNbDead _asescape_vectorcharacter)))) (Variables|Default|GetFontColor) (- (/ (.X (Math|Vector2D|BreakVector2D (Variables|Default|GetScreenDimensions))) 2.0) 7e+01) (/ (.Y (Math|Vector2D|BreakVector2D (Variables|Default|GetScreenDimensions))) 2e+01) (Variables|Default|GetFont) 0.8 false)
            ;[1 1 1] Draw number of Beamer Killed
            (HUD|DrawText (Utilities|String|ToString(Integer) (Variables|Default|GetNbBeamerKilled)) (Variables|Default|GetFontColor) (/ (.X (Math|Vector2D|BreakVector2D (Variables|Default|GetScreenDimensions))) 0.97) (/ (.Y (Math|Vector2D|BreakVector2D (Variables|Default|GetScreenDimensions))) 5.2) (Variables|Default|GetFont) 0.7 true)
            ;[1 1 1] Draw item logos
            (bind _asbp_escape_vector_character_c (Utilities|Casting|CastToBP_Escape_Vector_Character (Game|GetPlayerCharacter 0)))
            (if (Variables|/Game/Blueprints/BP_Escape_Vector_Character.BP_Escape_Vector_Character_C|Getitem_destroyAllLeechers _asbp_escape_vector_character_c)
              (HUD|DrawText "S" (Utilities|Struct|MakeLinearColor 0.0 255.0 0.0 255.0) (/ (.X (Math|Vector2D|BreakVector2D (Variables|Default|GetScreenDimensions))) 16.0) (/ (.Y (Math|Vector2D|BreakVector2D (Variables|Default|GetScreenDimensions))) 1.2) 0 2.0 false)
              (else
                (HUD|DrawText "S" (Utilities|Struct|MakeLinearColor 255.0 0.0 0.0 255.0) (/ (.X (Math|Vector2D|BreakVector2D (Variables|Default|GetScreenDimensions))) 16.0) (/ (.Y (Math|Vector2D|BreakVector2D (Variables|Default|GetScreenDimensions))) 1.2) 0 2.0 false)))
            (bind _asbp_escape_vector_character_c_2 (Utilities|Casting|CastToBP_Escape_Vector_Character (Game|GetPlayerCharacter 0)))
            (if (Variables|/Game/Blueprints/BP_Escape_Vector_Character.BP_Escape_Vector_Character_C|Getitem_speedBoost _asbp_escape_vector_character_c_2)
              (HUD|DrawText "W" (Utilities|Struct|MakeLinearColor 0.0 255.0 0.0 255.0) (/ (.X (Math|Vector2D|BreakVector2D (Variables|Default|GetScreenDimensions))) 16.0) (/ (.Y (Math|Vector2D|BreakVector2D (Variables|Default|GetScreenDimensions))) 1.25) _font 1.0 false)
              (elif (Variables|/Game/Blueprints/BP_Escape_Vector_Character.BP_Escape_Vector_Character_C|GetisSpeedBoosted _asbp_escape_vector_character_c_2)
                (HUD|DrawText "W" (Utilities|Struct|MakeLinearColor 0.0 255.0 255.0 255.0) (/ (.X (Math|Vector2D|BreakVector2D (Variables|Default|GetScreenDimensions))) 16.0) (/ (.Y (Math|Vector2D|BreakVector2D (Variables|Default|GetScreenDimensions))) 1.25) _font 1.0 false)
                (else
                  (HUD|DrawText "W" (Utilities|Struct|MakeLinearColor 255.0 0.0 0.0 255.0) (/ (.X (Math|Vector2D|BreakVector2D (Variables|Default|GetScreenDimensions))) 16.0) (/ (.Y (Math|Vector2D|BreakVector2D (Variables|Default|GetScreenDimensions))) 1.25) _font 1.0 false))))
            ;[1 1 1] Print Log
            (if (Variables|Default|GetprintLog)
              (HUD|DrawText _messagelog (Variables|Default|GetFontColor) (- (/ (.X (Math|Vector2D|BreakVector2D (Variables|Default|GetScreenDimensions))) 2.0) (* (Utilities|String|Len _messagelog) 7.1)) (/ (.Y (Math|Vector2D|BreakVector2D (Variables|Default|GetScreenDimensions))) 1.05) (Variables|Default|GetFont) 0.8 false)
              (Utilities|FlowControl|Delay 5.0)
              (Variables|Default|SetprintLog false))))))
    (:then_1
      ;[1 0.4197 0.4388] Verify if we need to change the crosshair and activate pannels.
      (bind _outactors_2 (Actor|GetAllActorsOfClass "/Game/Blueprints/BlueprintPanneau.BlueprintPanneau_C"))
      (for _array_element _outactors_2
        (Variables|Default|SetCurrentPanel _array_element)
        (bind (_closeenough _distancebetween) (CallFunction|CloseEnough (Variables|Default|GetDetectionRange) (Game|GetPlayerCharacter 0) (Variables|Default|GetCurrentPanel)))
        (if _closeenough
          (bind _visible (CallFunction|VerifyVisibility))
          (if _visible
            (Variables|Default|SetDistancePanel _distancebetween)
            (bind _asblueprintpanneau_c (Utilities|Casting|CastToBlueprintPanneau (Variables|Default|GetCurrentPanel)))
            (Variables|Default|SetCurrentPanel_BP _asblueprintpanneau_c)
            (Utilities|FlowControl|Sequence
              (:then_0
                (bind _isontherange (CallFunction|IsontheCrossRange (Transformation|GetActorLocation (Variables|Default|GetCurrentPanel)) (* (/ (Variables|Default|GetDetectionRange) (Variables|Default|GetDistancePanel)) 7.0)))
                (if _isontherange
                  (Variables|Default|Setcrosshair "/Game/Textures/T_CrossHair_Panelover.T_CrossHair_Panelover")
                  (Variables|/Game/Blueprints/BlueprintPanneau.BlueprintPanneau_C|SetAimedAt (Variables|Default|GetCurrentPanel_BP) true)))
              (:then_1
                (bind _isontherange_2 (CallFunction|IsontheCrossRange (Transformation|GetActorLocation (Variables|Default|GetCurrentPanel)) 1e+02))
                (if _isontherange_2
                  (if (not (Variables|/Game/Blueprints/BlueprintPanneau.BlueprintPanneau_C|GetOnPlatform (Variables|Default|GetCurrentPanel_BP)))
                    (Components|Animation|PlayAnimation (Variables|/Game/Blueprints/BlueprintPanneau.BlueprintPanneau_C|Get%20Panneau_Skeletal_Mesh (Variables|Default|GetCurrentPanel_BP)) "/Game/Assets/panneau/panneaux_redesign/AS_panneau_activation_02.AS_panneau_activation_02" false)
                    (Components|Timeline|SetPlayRate (Variables|/Game/Blueprints/BlueprintPanneau.BlueprintPanneau_C|Get%20Panneau_Skeletal_Mesh (Variables|Default|GetCurrentPanel_BP)) 1.0)
                    (Rendering|SetRenderCustomDepth (Variables|/Game/Blueprints/BlueprintPanneau.BlueprintPanneau_C|Get%20Panneau_Skeletal_Mesh (Variables|Default|GetCurrentPanel_BP)) true)
                    (Variables|/Game/Blueprints/BlueprintPanneau.BlueprintPanneau_C|SetActivated (Variables|Default|GetCurrentPanel_BP) true)))))))))
    (:then_2
      (bind _outactors_3 (Actor|GetAllActorsOfClass "/Game/Blueprints/BlueprintPanneau.BlueprintPanneau_C"))
      (for _array_element_2 _outactors_3
        (Variables|Default|SetCurrentPanel _array_element_2)
        (bind _closeenough_2 (CallFunction|CloseEnough (Variables|Default|GetDetectionRange) (Game|GetPlayerCharacter 0) (Variables|Default|GetCurrentPanel)))
        (if _closeenough_2
          (bind _asblueprintpanneau_c_2 (Utilities|Casting|CastToBlueprintPanneau (Variables|Default|GetCurrentPanel)))
          (Variables|Default|SetCurrentPanel_BP _asblueprintpanneau_c_2)
          (Utilities|FlowControl|Sequence
            (:then_0
              (if (Variables|/Game/Blueprints/BlueprintPanneau.BlueprintPanneau_C|GetAimedAt (Variables|Default|GetCurrentPanel_BP))
                (bind _isontherange_3 (CallFunction|IsontheCrossRange (Transformation|GetActorLocation (Variables|Default|GetCurrentPanel)) (* (/ (Variables|Default|GetDetectionRange) (Variables|Default|GetDistancePanel)) 7.0)))
                (if (not _isontherange_3)
                  (Variables|Default|Setcrosshair "/Game/Textures/Crosshair.crosshair")
                  (Variables|/Game/Blueprints/BlueprintPanneau.BlueprintPanneau_C|SetAimedAt (Variables|Default|GetCurrentPanel_BP) false))))
            (:then_1
              (if (Variables|/Game/Blueprints/BlueprintPanneau.BlueprintPanneau_C|GetActivated (Variables|Default|GetCurrentPanel_BP))
                (bind _isontherange_4 (CallFunction|IsontheCrossRange (Transformation|GetActorLocation (Variables|Default|GetCurrentPanel)) 1e+02))
                (if (not _isontherange_4)
                  (if (not (Variables|/Game/Blueprints/BlueprintPanneau.BlueprintPanneau_C|GetOnPlatform (Variables|Default|GetCurrentPanel_BP)))
                    (if (Variables|/Game/Blueprints/BlueprintPanneau.BlueprintPanneau_C|GetDelayCompleted (Variables|Default|GetCurrentPanel_BP))
                      (Components|Animation|PlayAnimation (Variables|/Game/Blueprints/BlueprintPanneau.BlueprintPanneau_C|Get%20Panneau_Skeletal_Mesh (Variables|Default|GetCurrentPanel_BP)) "/Game/Assets/panneau/panneaux_redesign/AS_panneau_activation_02.AS_panneau_activation_02" false)
                      (Components|Timeline|SetPlayRate (Variables|/Game/Blueprints/BlueprintPanneau.BlueprintPanneau_C|Get%20Panneau_Skeletal_Mesh (Variables|Default|GetCurrentPanel_BP)) -1.0)
                      (Variables|/Game/Blueprints/BlueprintPanneau.BlueprintPanneau_C|SetActivated (Variables|Default|GetCurrentPanel_BP) false)
                      (Rendering|SetRenderCustomDepth (Variables|/Game/Blueprints/BlueprintPanneau.BlueprintPanneau_C|Get%20Panneau_Skeletal_Mesh (Variables|Default|GetCurrentPanel_BP)) false))))))))))))

(event EventHitBoxBeginCursorOver
  (params (BoxName :type Name :default "None"))
  (bind _buttontexturehover (Variables|ButtonTexture|GetButtonTextureHover))
  (switch name BoxName
    (:Retry
      (Variables|ButtonTexture|SetRetryButtonTexture _buttontexturehover))
    (:Quit
      (Variables|ButtonTexture|SetQuitGameButtonTexture _buttontexturehover))
    (:ReturnToMain
      (Variables|ButtonTexture|SetReturnToMenuButtonTexture _buttontexturehover))
    (:Resume
      (Variables|ButtonTexture|SetResumeTextureButton _buttontexturehover))))

(event EventHitBoxEndCursorOver
  (params (BoxName :type Name :default "None"))
  (bind _buttontexturenormal (Variables|ButtonTexture|GetButtonTextureNormal))
  (switch name BoxName
    (:Retry
      (Variables|ButtonTexture|SetRetryButtonTexture _buttontexturenormal))
    (:Quit
      (Variables|ButtonTexture|SetQuitGameButtonTexture _buttontexturenormal))
    (:ReturnToMain
      (Variables|ButtonTexture|SetReturnToMenuButtonTexture _buttontexturenormal))
    (:Resume
      (Variables|ButtonTexture|SetResumeTextureButton _buttontexturenormal))))

(event EventHitBoxClick
  (params (BoxName :type Name :default "None"))
  (bind _buttontextureclick (Variables|ButtonTexture|GetButtonTextureClick))
  (switch name BoxName
    (:Retry
      (Variables|ButtonTexture|SetRetryButtonTexture _buttontextureclick))
    (:Quit
      (Variables|ButtonTexture|SetQuitGameButtonTexture _buttontextureclick))
    (:ReturnToMain
      (Variables|ButtonTexture|SetReturnToMenuButtonTexture _buttontextureclick))
    (:Resume
      (Variables|ButtonTexture|SetResumeTextureButton _buttontextureclick))))

(event EventBeginPlay
  (Input|EnableInput (Game|Player|GetOwningPlayerController))
  (Utilities|FlowControl|Delay 0.5)
  (CallFunction|SetBeamerRespawnPosRot))

(event Input|KeyboardEvents|P
  ;[1 1 1] Toggle Pause Menu
  (:Pressed
    (if (Variables|Default|GetTogglePauseMenu)
      (Variables|Default|SetTogglePauseMenu false)
      (else
        (Variables|Default|SetTogglePauseMenu true)
        (CallFunction|SetGametoPause)))))

(fn ConstructionScript
  (bind _returnvalue (Rendering|Material|CreateDynamicMaterialInstance "/Game/Materials/M_ShieldBar.M_ShieldBar" :!class /Script/Engine.KismetMaterialLibrary))
  (Variables|Default|SetShieldDynamicBar _returnvalue))

(fn SetGametoPause
  (bind _returnvalue (Game|GetPlayerController 0))
  (Variables|/Script/Engine.PlayerController|SetbShowMouseCursor _returnvalue true)
  (Variables|/Script/Engine.PlayerController|SetbEnableMouseOverEvents _returnvalue true)
  (Variables|/Script/Engine.PlayerController|SetbEnableClickEvents _returnvalue true)
  (Input|DisableInput _returnvalue _returnvalue)
  (Input|SetIgnoreLookInput _returnvalue true)
  (Game|SetGamePaused true))

(fn DrawCrosshair
  (params (Texture :type Texture%202D%20Object%20Reference))
  (bind _screendimensions (Variables|Default|GetScreenDimensions))
  (bind (_x _y) (Math|Vector2D|BreakVector2D _screendimensions))
  (Class|HUD|DrawTextureSimple Texture (- (/ _x 2.0) (Math|Conversions|ToFloat(Integer) (/ (Class|Texture2D|BlueprintGetSizeX Texture) 2))) (- (/ _y 2.0) (Math|Conversions|ToFloat(Integer) (/ (Class|Texture2D|BlueprintGetSizeY Texture) 2))) 1.0 false))

(fn BeamerKilled
  (CallFunction|PrintMessage "A Beamer has been Killed!")
  (Variables|Default|SetNbBeamerKilled (+ (Variables|Default|GetNbBeamerKilled) 1)))

(fn DrawButton
  (params (Texture :type Texture%202D%20Object%20Reference) (Position :type Vector%202D%20Structure) (HitBoxName :type Name) (Text :type String))
  (bind _returnvalue (Class|Texture2D|BlueprintGetSizeX Texture))
  (bind _returnvalue_2 (Class|Texture2D|BlueprintGetSizeY Texture))
  (bind (_x _y) (Math|Vector2D|BreakVector2D Position))
  (bind _returnvalue_3 (Math|Conversions|ToFloat(Integer) _returnvalue))
  (bind _returnvalue_4 (Math|Conversions|ToFloat(Integer) _returnvalue_2))
  (bind _returnvalue_5 (Math|Vector2D|MakeVector2D _returnvalue_3 _returnvalue_4))
  (bind _returnvalue_6 (/ _returnvalue_5 2.0))
  (bind _returnvalue_7 (+ Position _returnvalue_6))
  (bind (_x_2 _y_2) (Math|Vector2D|BreakVector2D _returnvalue_7))
  (Class|HUD|DrawTextureSimple Texture _x _y 1.0 false)
  (Class|HUD|AddHitBox Position _returnvalue_5 HitBoxName false)
  (HUD|DrawText Text (Variables|Default|GetFontColor) (- _x_2 (* (Utilities|String|Len Text) 7.5)) (- _y_2 2e+01) (Variables|Default|GetFont) 1.0 false))

(fn SetGametoUnPause
  (bind _returnvalue (Game|GetPlayerController 0))
  (Variables|/Script/Engine.PlayerController|SetbShowMouseCursor _returnvalue false)
  (Variables|/Script/Engine.PlayerController|SetbEnableMouseOverEvents _returnvalue false)
  (Variables|/Script/Engine.PlayerController|SetbEnableClickEvents _returnvalue false)
  (Input|DisableInput _returnvalue _returnvalue)
  (Input|SetIgnoreLookInput _returnvalue false)
  (Variables|Default|SetToggleRestartMenu false)
  (Variables|Default|SetTogglePauseMenu false)
  (Game|SetGamePaused false))

(fn DrawRestartMenu
  (bind _retrybuttontexture (Variables|ButtonTexture|GetRetryButtonTexture))
  (bind _screendimensions (Variables|Default|GetScreenDimensions))
  (bind _returnvalue (Class|Texture2D|BlueprintGetSizeX _retrybuttontexture))
  (bind _returnvalue_2 (Class|Texture2D|BlueprintGetSizeY _retrybuttontexture))
  (bind (_x _y) (Math|Vector2D|BreakVector2D _screendimensions))
  (bind _returnvalue_3 (/ _returnvalue_2 2))
  (bind _returnvalue_4 (/ _returnvalue 2))
  (bind _returnvalue_5 (/ _y 2.0))
  (bind _returnvalue_6 (/ _x 2.0))
  (bind _returnvalue_7 (Math|Conversions|ToFloat(Integer) _returnvalue_3))
  (bind _returnvalue_8 (Math|Conversions|ToFloat(Integer) _returnvalue_4))
  (bind _returnvalue_9 (- _returnvalue_6 _returnvalue_8))
  (bind _returnvalue_10 (- _returnvalue_5 _returnvalue_7))
  (CallFunction|DrawButton _retrybuttontexture (Math|Vector2D|MakeVector2D _returnvalue_9 (- _returnvalue_10 4e+01)) "Retry" "Retry")
  (CallFunction|DrawButton (Variables|ButtonTexture|GetQuitGameButtonTexture) (Math|Vector2D|MakeVector2D _returnvalue_9 (+ _returnvalue_10 8e+01)) "Quit" "Quit"))

(fn DrawDynamicBar
  (params (DynamicMaterial :type Material%20Instance%20Dynamic%20Object%20Reference) (ParameterName :type Name) (Value :type Float%20%28single-precision%29) (MaxValue :type Float%20%28single-precision%29) (Location :type Vector%202D%20Structure))
  (bind (_x _y) (Math|Vector2D|BreakVector2D Location))
  (Rendering|Material|SetScalarParameterValue DynamicMaterial ParameterName (* Value 1e+02) :!class /Script/Engine.MaterialInstanceDynamic)
  (Class|HUD|DrawMaterialSimple DynamicMaterial _x _y (* MaxValue 2.0) 25.0 1.0 false))

(fn IsontheCrossRange
  (params (Location :type Vector) (Rayon :type Float%20%28single-precision%29))
  (bind _returnvalue (Class|HUD|Project Location))
  (bind _screendimensions (Variables|Default|GetScreenDimensions))
  (bind _returnvalue_2 (/ _screendimensions 2.0))
  (bind (_x _y _z) (Math|Vector|BreakVector _returnvalue))
  (bind (_x_2 _y_2) (Math|Vector2D|BreakVector2D _returnvalue_2))
  (return (and (> _z 0.0) (< (Math|Float|Square (- _x _x_2) (- _y _y_2)) (Math|Float|Square Rayon)))))

(fn CloseEnough
  (params (Distance :type Float%20%28single-precision%29) (Actor%201 :type Actor%20Object%20Reference) (Actor%202 :type Actor%20Object%20Reference))
  (bind _returnvalue (Transformation|GetDistanceTo Actor%201 Actor%202))
  (if (<= _returnvalue 1e+02)
    (Variables|Default|SetCanDashToSpecificPanel false)
    (else
      (Variables|Default|SetCanDashToSpecificPanel (<= _returnvalue Distance))))
  (return (Variables|Default|GetCanDashToSpecificPanel) _returnvalue))

(fn DrawPauseMenu
  (bind _screendimensions (Variables|Default|GetScreenDimensions))
  (bind _resumetexturebutton (Variables|ButtonTexture|GetResumeTextureButton))
  (bind _returnvalue (Class|Texture2D|BlueprintGetSizeX _resumetexturebutton))
  (bind _returnvalue_2 (Class|Texture2D|BlueprintGetSizeY _resumetexturebutton))
  (bind (_x _y) (Math|Vector2D|BreakVector2D _screendimensions))
  (bind _returnvalue_3 (/ _returnvalue_2 2))
  (bind _returnvalue_4 (/ _returnvalue 2))
  (bind _returnvalue_5 (/ _y 2.0))
  (bind _returnvalue_6 (/ _x 2.0))
  (bind _returnvalue_7 (Math|Conversions|ToFloat(Integer) _returnvalue_3))
  (bind _returnvalue_8 (Math|Conversions|ToFloat(Integer) _returnvalue_4))
  (bind _returnvalue_9 (- _returnvalue_6 _returnvalue_8))
  (bind _returnvalue_10 (- _returnvalue_5 _returnvalue_7))
  (CallFunction|DrawButton _resumetexturebutton (Math|Vector2D|MakeVector2D _returnvalue_9 (- _returnvalue_10 2e+02)) "Resume" "Resume")
  (CallFunction|DrawButton (Variables|ButtonTexture|GetRetryButtonTexture) (Math|Vector2D|MakeVector2D _returnvalue_9 (- _returnvalue_10 8e+01)) "Retry" "Retry")
  (CallFunction|DrawButton (Variables|ButtonTexture|GetReturnToMenuButtonTexture) (Math|Vector2D|MakeVector2D _returnvalue_9 (+ _returnvalue_10 4e+01)) "ReturnToMain" "Main Menu")
  (CallFunction|DrawButton (Variables|ButtonTexture|GetQuitGameButtonTexture) (Math|Vector2D|MakeVector2D _returnvalue_9 (+ _returnvalue_10 2e+02)) "Quit" "Quit"))

(fn VerifyVisibility
  (bind (_outhit _returnvalue) (Collision|LineTraceByChannel (Transformation|GetActorLocation (Game|GetPlayerCharacter 0)) (Transformation|GetActorLocation (Variables|Default|GetCurrentPanel)) "TraceTypeQuery1" false 0 "None"))
  (if _returnvalue
    (Utilities|Casting|CastToBlueprintPanneau (.HitActor (Collision|BreakHitResult _outhit))
      (:then
        (Variables|Default|SetVisibility true))
      (:CastFailed
        (Variables|Default|SetVisibility false)))
    (return (Variables|Default|GetVisibility))))

(fn SetBeamerRespawnPosRot
  (bind _outactors (Actor|GetAllActorsOfClass "/Game/Blueprints/Beamer.Beamer_C"))
  (for _array_element _outactors
    (bind _asbeamer_c (Utilities|Casting|CastToBeamer _array_element))
    (Utilities|Array|Add (Variables|Default|GetBeamerPos) (Transformation|GetActorLocation _array_element))
    (Utilities|Array|Add (Variables|Default|GetBeamerRotations) (Transformation|GetActorRotation _array_element))
    (Utilities|Array|Add (Variables|Default|GetBeamerCheckpoint) (Variables|/Game/Blueprints/Beamer.Beamer_C|GetCheckpoint_Association _asbeamer_c))))

(fn RespawnBeamerCheckpoint
  (bind _asbp_escape_vector_character_c (Utilities|Casting|CastToBP_Escape_Vector_Character (Game|GetPlayerCharacter 0)))
  (bind _outactors (Actor|GetAllActorsOfClass "/Game/Blueprints/Beamer.Beamer_C"))
  (for _array_element _outactors
    (Actor|DestroyActor _array_element))
  (for (_array_element_2 _array_index) (Variables|Default|GetBeamerPos)
    (if (>= (Utilities|Array|Get(acopy) (Variables|Default|GetBeamerCheckpoint) _array_index) (Variables|/Game/Blueprints/BP_Escape_Vector_Character.BP_Escape_Vector_Character_C|GetCheckPointNumber _asbp_escape_vector_character_c))
      (Game|SpawnActorfromClass "/Game/Blueprints/Beamer.Beamer_C" (Math|Transform|MakeTransform _array_element_2 (Utilities|Array|Get(acopy) (Variables|Default|GetBeamerRotations) _array_index)) true))))

(fn PrintMessage
  (params (message :type String))
  (Variables|Default|SetMessageLog message)
  (Variables|Default|SetprintLog true))

(fn GetShipCitizen
  (return 0))

(fn GetShipShield
  (return 0.0 0.0))

(fn GetShipSpeed
  (return 0.0))