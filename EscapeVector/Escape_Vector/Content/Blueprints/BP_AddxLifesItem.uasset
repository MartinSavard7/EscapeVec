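; BP_AddxLifesItem is a pickup that restores one life to the player.
; When the player character overlaps Box1, it casts to BP_Escape_Vector_Character and lowers that character's INbDead death counter by one, clamped at zero.
; The item then destroys itself and prints a confirmation message, and it is consumed even if the counter is already at zero.
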(event OnComponentBeginOverlap(Box1)
  (params (OtherActor :type Actor%20Object%20Reference) (OtherComp :type Primitive%20Component%20Object%20Reference) (OtherBodyIndex :type Integer) (bFromSweep :type Boolean) (SweepResult :type Hit%20Result%20Structure%20%28by%20ref%29))
  (bind _returnvalue (Game|GetPlayerCharacter 0))
  ;[1 1 1] Add 1 life to the player
  (if (== OtherActor _returnvalue)
    (bind _asbp_escape_vector_character_c (Utilities|Casting|CastToBP_Escape_Vector_Character _returnvalue))
    (if (< (- (Variables|/Script/Escape_Vector.Escape_VectorCharacter|GetiNbDead _asbp_escape_vector_character_c) 1.0) 0.0)
      (Variables|/Script/Escape_Vector.Escape_VectorCharacter|SetiNbDead _asbp_escape_vector_character_c 0.0)
      (else
        (Variables|/Script/Escape_Vector.Escape_VectorCharacter|SetiNbDead _asbp_escape_vector_character_c (- (Variables|/Script/Escape_Vector.Escape_VectorCharacter|GetiNbDead _asbp_escape_vector_character_c) 1.0))))
    (Actor|DestroyActor)
    (Development|PrintString "One life restored!")))

(fn ConstructionScript)