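; Beamer enemy actor that idles, plays a ship-attack animation on demand, and dies when the player pawn touches it.
; On player overlap it notifies MyHUD, plays its death animation, disables collision, toggles the character's text render for a second and destroys itself after a delay.
; Other overlaps can turn it toward an overlapping Ship.
; AttackShip and ReturntoRest switch the idle flag that Tick checks to play the idle animation.
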(event OnComponentBeginOverlap(CollisionBox)
  (params (OtherActor :type Actor%20Object%20Reference) (OtherComp :type Primitive%20Component%20Object%20Reference) (OtherBodyIndex :type Integer) (bFromSweep :type Boolean) (SweepResult :type Hit%20Result%20Structure%20%28by%20ref%29))
  (bind _overlappingactors (Collision|GetOverlappingActors "/Game/Blueprints/Ship.Ship_C" :!class /Script/Engine.Actor))
  (bind _item (Utilities|Array|Get(acopy) _overlappingactors))
  ;[1 1 1] Called When the player hits the Beamer
  (if (== (Game|Player|GetPlayerPawn 0) OtherActor)
    (bind _asmyhud_c (Utilities|Casting|CastToMyHUD (HUD|GetHUD (Game|GetPlayerController 0))))
    (Default|BeamerKilled _asmyhud_c)
    (Development|PrintString "KILL!")
    (Variables|Default|SetisOnIdleState false)
    (Utilities|FlowControl|Sequence
      (:then_0
        (Components|Animation|PlayAnimation (Variables|Default|GetBeamerSkeletalMesh) "/Game/Character/Anim_sets/AS_mort.AS_mort" false)
        (Collision|SetCollisionEnabled (Variables|Default|GetCollisionBox) "NoCollision")
        (Utilities|FlowControl|Delay 2.0)
        (Actor|DestroyActor))
      (:then_1
        (if (== (Game|Player|GetPlayerPawn 0) OtherActor)
          (bind _asbp_escape_vector_character_c (Utilities|Casting|CastToBP_Escape_Vector_Character OtherActor))
          (Rendering|ToggleVisibility (Variables|/Game/Blueprints/BP_Escape_Vector_Character.BP_Escape_Vector_Character_C|GetTextRender1 _asbp_escape_vector_character_c) false)
          (Utilities|FlowControl|Delay 1.0)
          (Rendering|ToggleVisibility (Variables|/Game/Blueprints/BP_Escape_Vector_Character.BP_Escape_Vector_Character_C|GetTextRender1 _asbp_escape_vector_character_c) false))))
    (else
      ;[1 1 1] Called when the Ship hits the Beamer
      (if (== OtherActor _item)
        (Transformation|SetActorRelativeRotation (Math|Rotator|FindLookatRotation (Transformation|GetActorLocation) (Transformation|GetActorLocation _item)))))))

(event EventBeginPlay
  (Variables|Default|SetisOnIdleState true))

(event EventTick
  (params (DeltaSeconds :type Float%20%28single-precision%29))
  ;[1 1 1] Play Idle Animation
  (if (Variables|Default|GetisOnIdleState)
    (Components|Animation|PlayAnimation (Variables|Default|GetBeamerSkeletalMesh) "/Game/Character/Anim_sets/AS_anguille.AS_anguille" true)))

(fn ConstructionScript)

(fn AttackShip
  (Variables|Default|SetisOnIdleState false)
  (Components|Animation|PlayAnimation (Variables|Default|GetBeamerSkeletalMesh) "/Game/Character/Anim_sets/AS_attack_ship.AS_attack_ship" true))

(fn ReturntoRest
  (Variables|Default|SetisOnIdleState true))