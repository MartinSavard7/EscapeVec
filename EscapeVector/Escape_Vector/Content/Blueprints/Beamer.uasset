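; Beamer enemy actor that loops an idle animation until the player kills it.
; A player hit plays the death animation, launches it along the dash direction at dash speed, then dissolves it via dynamic material and notifies the HUD.
; Tick drives knockback, dissolve and delayed destruction; certain non-player collisions zero the velocity.
; KillSphere briefly sets the player's KillBeamer flag on entry for the kill animation.
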(event OnComponentBeginOverlap(CollisionBox)
  (params (OtherActor :type Actor%20Object%20Reference) (OtherComp :type Primitive%20Component%20Object%20Reference) (OtherBodyIndex :type Integer) (bFromSweep :type Boolean) (SweepResult :type Hit%20Result%20Structure%20%28by%20ref%29))
  ;[1 1 1] Called When the player hits the Beamer
  (if (== (Game|Player|GetPlayerPawn 0) OtherActor)
    (Components|Animation|PlayAnimation (Variables|Default|GetBeamerSkeletalMesh) "/Game/Character/Anim_sets/AS_Beamer_V2/AS_mort_V2.AS_mort_V2" true)
    (bind _asbp_escape_vector_character_c (Utilities|Casting|CastToBP_Escape_Vector_Character (Game|GetPlayerCharacter 0)))
    (Variables|Default|SetKillForceDirection (Variables|/Game/Blueprints/BP_Escape_Vector_Character.BP_Escape_Vector_Character_C|GetDirectionDash _asbp_escape_vector_character_c))
    (Variables|Default|SetVelocity (Variables|/Game/Blueprints/BP_Escape_Vector_Character.BP_Escape_Vector_Character_C|GetStartSpeed _asbp_escape_vector_character_c))
    (Variables|Default|SetisHitByPlayer true)
    (Utilities|FlowControl|Delay 1.0)
    (Variables|Default|SetdestroyBeamer true)
    (bind _asmyhud_c (Utilities|Casting|CastToMyHUD (HUD|GetHUD (Game|GetPlayerController 0))))
    (Default|BeamerKilled _asmyhud_c)
    (else
      ;[1 1 1] Called when the Ship hits the Beamer
      (if (not (== OtherActor (Utilities|Array|Get(acopy) (Collision|GetOverlappingActors "/Game/Blueprints/Ship.Ship_C" :!class /Script/Engine.Actor))))
        (Variables|Default|SetVelocity 0.0)))))

(event OnComponentBeginOverlap(KillSphere)
  (params (OtherActor :type Actor%20Object%20Reference) (OtherComp :type Primitive%20Component%20Object%20Reference) (OtherBodyIndex :type Integer) (bFromSweep :type Boolean) (SweepResult :type Hit%20Result%20Structure%20%28by%20ref%29))
  ;[1 1 1] Lorsque le joueur entre dans sphere sa valeur "killBeamer" est mis a true, donc l'anim de kill doit jouer
  (if (== (Game|Player|GetPlayerPawn 0) OtherActor)
    (bind _asbp_escape_vector_character_c (Utilities|Casting|CastToBP_Escape_Vector_Character OtherActor))
    (Variables|/Game/Blueprints/BP_Escape_Vector_Character.BP_Escape_Vector_Character_C|SetkillBeamer _asbp_escape_vector_character_c true)
    (Utilities|FlowControl|Delay 1.0)
    (Variables|/Game/Blueprints/BP_Escape_Vector_Character.BP_Escape_Vector_Character_C|SetkillBeamer _asbp_escape_vector_character_c false)))

(event EventBeginPlay
  ;[1 1 1] Play Idle Animation
  (Components|Animation|PlayAnimation (Variables|Default|GetBeamerSkeletalMesh) "/Game/Character/Anim_sets/AS_Beamer_V2/AS_anguille_V2.AS_anguille_V2" true))

(event EventTick
  (params (DeltaSeconds :type Float%20%28single-precision%29))
  (bind _self self)
  ;[1 1 1] Move in player direction
  (if (Variables|Default|GetisHitByPlayer)
    (Transformation|SetActorRelativeLocation _self (+ (Transformation|GetActorLocation _self) (* (Variables|Default|GetKillForceDirection) (/ (Variables|Default|GetVelocity) 7.0))) true)
    (if (Variables|Default|GetdestroyBeamer)
      (Variables|Default|SetDissolve (- (Variables|Default|GetDissolve) 0.05))
      (Rendering|Material|SetScalarParameterValue (Variables|Default|GetDynamicMaterial) "DissolveValue" (Variables|Default|GetDissolve) :!class /Script/Engine.MaterialInstanceDynamic)
      (Utilities|FlowControl|Delay 3.0)
      (Actor|DestroyActor))))

(fn ConstructionScript
  (bind _returnvalue (Rendering|Material|CreateDynamicMaterialInstance (Variables|Default|GetBeamerSkeletalMesh) 0 0 :!class /Script/Engine.PrimitiveComponent))
  (Variables|Default|SetDynamicMaterial _returnvalue))

(fn AttackShip
  (if (Variables|Default|GetisHitByPlayer)
    (Components|Animation|PlayAnimation (Variables|Default|GetBeamerSkeletalMesh) "/Game/Character/Anim_sets/AS_Beamer_V2/AS_attack_ship_V2.AS_attack_ship_V2" true)))